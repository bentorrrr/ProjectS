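; BP_QuestGiver is a quest giver that offers the quest named by its QuestData row to the main player character.
; GiveQuest runs on BeginPlay and queries the player's ACQuestLog component for that quest's active and completed state.
; It adds the quest only when it is not active and its completed-quest query reports TurnedIn as true.
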(event `self.ReceiveBeginPlay`
  (`self.GiveQuest`))

(event `GiveQuest`
  (bind (_questdata_datatable _questdata_rowname) (break `DataTableRowHandle` (`self.QuestData`)))
  (bind (_questdata_datatable_2 _questdata_rowname_2) (break `DataTableRowHandle` (`self.QuestData`)))
  (bind _ac_questlog (`/Game/ThirdPerson/Blueprints/BP_MainCharacter.AC_QuestLog` (`/Game/QuestSystem/Interaction/BPFL_CommonFunction.GetMainPlayerCharacter`)))
  (if (and (not (`/Game/QuestSystem/AC_QuestLog.QueryActiveQuest` _ac_questlog _questdata_rowname_2)) (`.TurnedIn` (`/Game/QuestSystem/AC_QuestLog.QueryCompletedQuests` _ac_questlog _questdata_rowname_2)))
    (`/Game/QuestSystem/AC_QuestLog.AddNewQuest` (`/Game/ThirdPerson/Blueprints/BP_MainCharacter.AC_QuestLog` (`/Game/QuestSystem/Interaction/BPFL_CommonFunction.GetMainPlayerCharacter`)) _questdata_rowname)))

(fn `UserConstructionScript`)