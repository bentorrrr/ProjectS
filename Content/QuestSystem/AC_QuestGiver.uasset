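; AC_QuestGiver is a quest-giver component that handles interaction with its owning actor.
; InteractWith asks the player's ACQuestLog whether the quest row named in QuestData is already active, calling DisplayQuest if not and printing a notice otherwise.
; Both branches return the owner's display name.
; DisplayQuest is an empty stub, and the event graph holds only disabled default events.
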(fn `DisplayQuest`)

(fn `InteractWith`
  (returns (ObjectiveID :type String))
  (bind (_questdata_datatable _questdata_rowname) (break `DataTableRowHandle` (`self.QuestData`)))
  (bind _returnvalue (`KismetSystemLibrary.GetDisplayName` (`self.GetOwner`)))
  (if (not (`/Game/QuestSystem/AC_QuestLog.QueryActiveQuest` (`/Game/ThirdPerson/Blueprints/BP_MainCharacter.AC_QuestLog` (`/Game/QuestSystem/Interaction/BPFL_CommonFunction.GetMainPlayerCharacter`)) _questdata_rowname))
    (`self.DisplayQuest`)
    (return _returnvalue)
    (else
      (`KismetSystemLibrary.PrintString` "Already on quest")
      (return _returnvalue))))