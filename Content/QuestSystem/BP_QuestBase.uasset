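; BP_QuestBase tracks one quest's progress through staged objectives, loading its definition from DT_QuestDetails by QuestID.
; It listens for objective ID events from the main player character, increments capped per-objective counts and broadcasts each change.
; A finished objective shows a notification widget; when all are done, the next stage loads.
; After the last stage it marks itself completed and, if AutoAccept is set, completes the quest in the player's quest log.
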(event `self.ReceiveBeginPlay`
  (`self.GetQuestDetails`)
  (add `/Game/ThirdPerson/Blueprints/BP_MainCharacter.OnObjectiveIDCalled` (`/Game/QuestSystem/Interaction/BPFL_CommonFunction.GetMainPlayerCharacter`) (`|CreateDelegate` :!event `On Objective IDHeard`))
  (`KismetSystemLibrary.Delay` 1.0)
  (bind _arecomplete (`self.AreAllObjectiveComplete`))
  (set `self.IsCompleted` _arecomplete))

(fn `AreAllObjectiveComplete`
  (returns (AreComplete :type Boolean))
  (locals (Local_AllCompleted :type Boolean :default true))
  (for _array_element (`.Objectives_24_3297965042C809E8004924A02A021176` (break `/Game/QuestSystem/S_StageDetails` (`self.CurrentStageDetail`)))
    (bind (_objectivename _description _type _objectiveid) (break `/Game/QuestSystem/S_ObjectiveDetails` _array_element))
    (if (not (>= (`BlueprintMapLibrary.Map_Find` (`self.CurrentObjectiveProgress`) _objectiveid) (`.Quantity_18_6697BF7C415B9A3AB339F29FF5CFCD74` (break `/Game/QuestSystem/S_ObjectiveDetails` (`self.GetObjectiveDetailsByID` _objectiveid)))))
      (bind _output_get (set `local.Local_AllCompleted` false))
      (return _output_get)))
  (return (`local.Local_AllCompleted`)))

(fn `GetObjectiveDetailsByID`
  (params (ObjectiveID :type String))
  (returns (ArrayElement :type "/Game/QuestSystem/S_ObjectiveDetails Structure"))
  (for _array_element (`.Objectives_24_3297965042C809E8004924A02A021176` (break `/Game/QuestSystem/S_StageDetails` (`self.CurrentStageDetail`)))
    (if (`KismetStringLibrary.EqualEqual_StrStr` ObjectiveID (`.ObjectiveID_12_68C0FBB44B8AF320FC02A38D36DF9976` (break `/Game/QuestSystem/S_ObjectiveDetails` _array_element)))
      (return _array_element))))

(fn `GetQuestDetails`
  (bind _returnvalue (`|GetDataTableRow` "/Game/QuestSystem/DT_QuestDetails.DT_QuestDetails" (`self.QuestID`))
    (:`then`
      (bind _output_get (set `self.QuestDetails` _returnvalue))
      (bind _output_get_2 (set `self.CurrentStageDetail` (`|GetArrayItem` (`.Stages_14_48BCC833408D5BB0F07B1FA57CB2DE1B` (break `/Game/QuestSystem/S_QuestDetails` _output_get)) (`self.CurrentStage`))))
      (`BlueprintMapLibrary.Map_Clear` (`self.CurrentObjectiveProgress`))
      (for _array_element (`.Objectives_24_3297965042C809E8004924A02A021176` (break `/Game/QuestSystem/S_StageDetails` _output_get_2))
        (`BlueprintMapLibrary.Map_Add` (`self.CurrentObjectiveProgress`) (`.ObjectiveID_12_68C0FBB44B8AF320FC02A38D36DF9976` (break `/Game/QuestSystem/S_ObjectiveDetails` _array_element)))))))

(fn `IsObjectiveComplete`
  (params (ObjectiveID :type String))
  (bind (_questdetails_questid _questdetails_questname _questdetails_logdescription _questdetails_trackingdescription _questdetails_ismainquest _questdetails_stages) (break `/Game/QuestSystem/S_QuestDetails` (`self.QuestDetails`)))
  (bind (_objectivename _description _type _objectiveid _quantity) (break `/Game/QuestSystem/S_ObjectiveDetails` (`self.GetObjectiveDetailsByID` ObjectiveID)))
  (if (>= (`BlueprintMapLibrary.Map_Find` (`self.CurrentObjectiveProgress`) (`local.ObjectiveID`)) _quantity)
    (bind _returnvalue (`|CreateWidget` "/Game/QuestSystem/UIs/W_QuestNotification.W_QuestNotification_C" null _description))
    (`UserWidget.AddToViewport` _returnvalue 0)
    (bind _arecomplete (`self.AreAllObjectiveComplete`))
    (if _arecomplete
      (bind _result (`/Engine/EditorBlueprintResources/StandardMacros.IncrementInt` (`self.CurrentStage`))
        (:`  `
          (if (`KismetArrayLibrary.Array_IsValidIndex` _questdetails_stages _result)
            (`self.GetQuestDetails`)
            (else
              (set `self.IsCompleted` true)
              (if (`.AutoAccept_16_D5281AF04738331DE957AF852DA9A794` (break `/Game/QuestSystem/S_QuestDetails` (`self.QuestDetails`)))
                (`/Game/QuestSystem/AC_QuestLog.CompleteQuest` (`/Game/ThirdPerson/Blueprints/BP_MainCharacter.AC_QuestLog` (`/Game/QuestSystem/Interaction/BPFL_CommonFunction.GetMainPlayerCharacter`)) (`self.QuestID`))))))))))

(fn `On Objective IDHeard`
  (params (ObjectiveID :type String))
  (bind (_value _returnvalue) (`BlueprintMapLibrary.Map_Find` (`self.CurrentObjectiveProgress`) ObjectiveID))
  (if _returnvalue
    (if (< _value (`.Quantity_18_6697BF7C415B9A3AB339F29FF5CFCD74` (break `/Game/QuestSystem/S_ObjectiveDetails` (`self.GetObjectiveDetailsByID` ObjectiveID))))
      (`BlueprintMapLibrary.Map_Add` (`self.CurrentObjectiveProgress`) (`local.ObjectiveID`) (+ _value 1))
      (`self.IsObjectiveComplete` (`local.ObjectiveID`))
      (`self.OnObjectiveHeard`)
      (return))
    (else
      (return))))

(fn `UserConstructionScript`)