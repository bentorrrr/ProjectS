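; Quest log component that tracks active and completed quests, each active quest backed by a spawned BP_QuestBase actor.
; TurnInQuest adds currency rewards to the game instance, then CompleteQuest updates the lists and either handles the tracker or, without one, fires OnQuestCompleted.
; TrackQuest toggles or retargets a W_Tracker widget.
; Query functions report quest status and DT_QuestDetails prerequisites, while hardcoded completions spawn auto-accept BP_QuestGivers for follow-up quests.
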(fn `AddNewQuest`
  (params (QuestID :type Name) (CurrentStage :type Integer))
  (returns (Quest :type "/Game/QuestSystem/BP_QuestBase Object Reference"))
  (`KismetArrayLibrary.Array_AddUnique` (`self.CurrentActiveQuest`) QuestID)
  (bind _returnvalue (`|SpawnActorFromClass` "/Game/QuestSystem/BP_QuestBase.BP_QuestBase_C" (`KismetMathLibrary.MakeTransform` (0.0 0.0 0.0)) "Undefined" "MultiplyWithRoot" null QuestID CurrentStage null))
  (`KismetArrayLibrary.Array_Add` (`self.CurrentQuests`) _returnvalue)
  (return _returnvalue))

(fn `CompleteQuest`
  (params (QuestID :type Name))
  (`KismetArrayLibrary.Array_AddUnique` (`self.CompletedQuest`) QuestID)
  (`KismetArrayLibrary.Array_RemoveItem` (`self.CurrentActiveQuest`) QuestID)
  (bind _questactor (`self.GetQuestActor` QuestID))
  (`KismetArrayLibrary.Array_RemoveItem` (`self.CurrentQuests`) _questactor)
  (set `/Game/QuestSystem/BP_QuestBase.IsTurnedIn` true _questactor)
  (bind _tracker (`self.Tracker`)
    (:`then`
      (if (== QuestID (`/Game/QuestSystem/BP_QuestBase.QuestID` (`/Game/QuestSystem/UIs/W_Tracker.QuestActor` _tracker)))
        (`Widget.RemoveFromParent` (`self.Tracker`))))
    (:`else`
      (`self.OnQuestCompleted` _questactor QuestID)))
  ;[1 1 1] Spawning Auto accept Quest
  (if (== QuestID "002")
    (`|SpawnActorFromClass` "/Game/QuestSystem/BP_QuestGiver.BP_QuestGiver_C" (`KismetMathLibrary.MakeTransform` (0.0 0.0 0.0)) "Undefined" "MultiplyWithRoot" null (make `DataTableRowHandle` "/Game/QuestSystem/DT_QuestDetails.DT_QuestDetails" "003") null)
    (else
      ;[1 1 1] Spawning Auto accept Quest
      (if (== QuestID "004")
        (`|SpawnActorFromClass` "/Game/QuestSystem/BP_QuestGiver.BP_QuestGiver_C" (`KismetMathLibrary.MakeTransform` (0.0 0.0 0.0)) "Undefined" "MultiplyWithRoot" null (make `DataTableRowHandle` "/Game/QuestSystem/DT_QuestDetails.DT_QuestDetails" "005") null)))))

(fn `GetQuestActor`
  (params (QuestID :type Name))
  (returns (QuestActor :type "/Game/QuestSystem/BP_QuestBase Object Reference"))
  (for _array_element (`self.CurrentQuests`)
    (if (== (`/Game/QuestSystem/BP_QuestBase.QuestID` _array_element) QuestID)
      (return _array_element))))

(fn `QueryActiveQuest`
  (params (QuestID :type Name))
  (returns (ReturnValue :type Boolean))
  (return (`KismetArrayLibrary.Array_Contains` (`self.CurrentActiveQuest`) QuestID)))

(fn `QueryCompletedQuests`
  (params (QuestID :type Name))
  (returns (ReturnValue :type Boolean) (TurnedIn :type Boolean))
  (bind _returnvalue (`KismetArrayLibrary.Array_Contains` (`self.CompletedQuest`) QuestID))
  (if (!= QuestID "0")
    (bind _questactor (`self.GetQuestActor` QuestID))
    (`/Engine/EditorBlueprintResources/StandardMacros.IsValid` _questactor
      (:`Is Valid`
        (return _returnvalue (`/Game/QuestSystem/BP_QuestBase.IsTurnedIn` _questactor)))
      (:`Is Not Valid`
        (return _returnvalue true)))
    (else
      (return true true))))

(fn `QueryPreviousQuestID`
  (params (QuestID :type Name))
  (returns (PreviousQuestID :type Name))
  (bind _returnvalue (`|GetDataTableRow` "/Game/QuestSystem/DT_QuestDetails.DT_QuestDetails" QuestID)
    (:`then`
      (return (`KismetStringLibrary.Conv_StringToName` (`KismetTextLibrary.Conv_TextToString` (`.PerviousQuestID_19_853C1F2C48478FF1D1DDF192EE66B650` (break `/Game/QuestSystem/S_QuestDetails` _returnvalue))))))))

(fn `TrackQuest`
  (params (QuestActor :type "/Game/QuestSystem/BP_QuestBase Object Reference"))
  (bind _tracker (`self.Tracker`))
  (bind _tracker_2 (`self.Tracker`))
  (`self.Tracker`
    (:`then`
      (if (== (`/Game/QuestSystem/UIs/W_Tracker.QuestActor` (`self.Tracker`)) QuestActor)
        (set `/Game/QuestSystem/UIs/W_Tracker.QuestActor` null _tracker)
        (`Widget.RemoveFromParent` _tracker)
        (else
          (`/Game/QuestSystem/UIs/W_Tracker.Update` _tracker_2 QuestActor)
          (`UserWidget.AddToViewport` _tracker_2 -1))))
    (:`else`
      (bind _returnvalue (`|CreateWidget` "/Game/QuestSystem/UIs/W_Tracker.W_Tracker_C" null QuestActor))
      (bind _output_get (set `self.Tracker` _returnvalue))
      (`UserWidget.AddToViewport` _output_get -1))))

(fn `TurnInQuest`
  (params (QuestID :type Name))
  (`|ExecutionSequence`
    (:`then_0`
      (bind _questactor (`self.GetQuestActor` QuestID))
      (bind _asbp_main_game_instance (cast `/Game/Utils/BP_MainGameInstance` (`GameplayStatics.GetGameInstance`)))
      (set `/Game/Utils/BP_MainGameInstance.PlayerCurrency` (+ (`/Game/Utils/BP_MainGameInstance.PlayerCurrency` _asbp_main_game_instance) (`.CurrencyRewards_21_19200C3F4F8DD6F89EF3909E79929DA8` (break `/Game/QuestSystem/S_StageDetails` (`/Game/QuestSystem/BP_QuestBase.CurrentStageDetail` _questactor)))) _asbp_main_game_instance))
    (:`then_1`
      (`self.CompleteQuest` QuestID))))