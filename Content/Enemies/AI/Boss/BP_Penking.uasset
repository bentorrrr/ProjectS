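; BP_Penking is a boss enemy that adds a health bar on spawn and ragdolls before being destroyed on death.
; Attack1 sphere-traces forward to damage a pawn with a hit effect.
; Attack2 spawns a random number of melee Penknights at traced points nearby, and Attack3 triggers a delayed stomp AOE that damages overlapping actors.
; Attacks set per-attack flags, while block and damage-response handlers only print debug text.
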(event `self.ReceiveBeginPlay`
  (`parent.ReceiveBeginPlay`)
  (bind _returnvalue (`|CreateWidget` "/Game/DamageSystem/W_BossHealthBar.W_BossHealthBar_C" null self))
  (`UserWidget.AddToViewport` _returnvalue 0))

(event `CustomEvent`
  (bind _mesh (`self.Mesh`))
  ;[1 1 1] Damage Response
  (`KismetSystemLibrary.PrintString` "Dead")
  (`PrimitiveComponent.SetSimulatePhysics` _mesh true)
  (`PrimitiveComponent.SetCollisionEnabled` _mesh "PhysicsOnly")
  (`NavMovementComponent.StopActiveMovement` (`self.CharacterMovement`))
  (bind _asaic_tree_boss (cast `/Game/Enemies/AI/Boss/AIC_Tree_Boss` (`self.GetController`)))
  (`Controller.UnPossess` _asaic_tree_boss)
  (`KismetSystemLibrary.Delay` 2.0)
  (`self.K2_DestroyActor`)
  (`Widget.RemoveFromParent` (stale `self.ReceiveBeginPlay` _returnvalue)))

(event `CustomEvent_1`
  (params (CanBeParried :type Boolean))
  ;[1 1 1] Damage Response
  (`KismetSystemLibrary.PrintString` "Blocked"))

(event `CustomEvent_2`
  (params (DamageResponse :type "/Game/DamageSystem/E_DamageResponse Enum" :default "NewEnumerator0"))
  ;[1 1 1] Damage Response
  (`KismetSystemLibrary.PrintString` (`|GetEnumeratorNameAsString` DamageResponse)))

(event `/Game/Enemies/AI/Boss/BPI_BossAI.Attack1`
  (bind _returnvalue (`self.K2_GetActorLocation`))
  ;[1 1 1] Basic Attack
  (`KismetSystemLibrary.PrintString` "Hello 1")
  (if (not (`/Game/DamageSystem/BPC_DamageSystem.IsDead` (`self.BPC_DamageSystem`)))
    (set `self.IsAttacking1` true)
    (bind (_outhit _returnvalue_2) (`KismetSystemLibrary.SphereTraceSingleForObjects` :`Start` _returnvalue :`End` (+ _returnvalue (* (`self.GetActorForwardVector`) 1000.0)) :`Radius` 500.0 :`ObjectTypes` (`|MakeArray` "ObjectTypeQuery3" :!type "EObjectTypeQuery Enum") :`TraceColor` (struct :`G` 0.236161 :`B` 1.0 :`A` 1.0) :`TraceHitColor` (struct :`R` 1.0 :`G` 0.739583 :`B` 0.899609 :`A` 1.0) :`DrawTime` 2.0))
    (if _returnvalue_2
      (bind (_bblockinghit _binitialoverlap _time _distance _location _impactpoint _normal _impactnormal _physmat _hitactor) (`GameplayStatics.BreakHitResult` _outhit))
      (message `/Game/DamageSystem/BPI_Damagable.TakeDamage` _hitactor (make `/Game/DamageSystem/S_DamageInfo` 10.0 "NewEnumerator1" "NewEnumerator1"))
      (`NiagaraFunctionLibrary.SpawnSystemAtLocation` "/Game/Effects/NS_EnemyHit.NS_EnemyHit" _location))))

(event `/Game/Enemies/AI/Boss/BPI_BossAI.Attack2`
  (bind _randomlocation (`NavigationSystemV1.K2_GetRandomReachablePointInRadius` (`self.K2_GetActorLocation`) (`self.SpawnRadius`) null null))
  (set `self.IsAttacking2` true)
  (for _ (range (+ (`KismetMathLibrary.RandomInteger` 5) 1))
    (bind (_outhit _returnvalue) (`KismetSystemLibrary.LineTraceSingle` _randomlocation (* _randomlocation (1.0 1.0 -1000.0)) "TraceTypeQuery1"))
    (if _returnvalue
      (`|SpawnActorFromClass` "/Game/Enemies/AI/EnemyClasses/BP_Penknight_Melee.BP_Penknight_Melee_C" (`KismetMathLibrary.MakeTransform` (`.Location` (`GameplayStatics.BreakHitResult` _outhit))) "AdjustIfPossibleButAlwaysSpawn" "MultiplyWithRoot" null false 0 "" 10.0 self))))

(event `/Game/Enemies/AI/Boss/BPI_BossAI.Attack3`
  (`KismetSystemLibrary.PrintString` "Hello 3")
  (set `self.IsAttacking3` true)
  (`KismetSystemLibrary.Delay` 1.0)
  (bind _returnvalue (`|SpawnActorFromClass` "/Game/DamageSystem/AOE/BP_PenKingStomp.BP_PenKingStomp_C" (`self.GetTransform`) "Undefined" "MultiplyWithRoot" null 500.0 true true false self))
  (add `/Game/DamageSystem/AOE/BP_AOE_Base.OnAOEOverlapActor` _returnvalue (delegate `Damaging AOE Actor`))
  (`/Game/DamageSystem/AOE/BP_AOE_Base.Trigger` _returnvalue)
  (`KismetSystemLibrary.Delay` 2.0))

(event `Damaging AOE Actor`
  (params (Actor :type "Actor Object Reference"))
  (message `/Game/DamageSystem/BPI_Damagable.TakeDamage` Actor (make `/Game/DamageSystem/S_DamageInfo` 10.0 "NewEnumerator1" "NewEnumerator1"))
  (`KismetSystemLibrary.PrintString` (`KismetSystemLibrary.GetDisplayName` Actor)))

(fn `UserConstructionScript`
  (`parent.UserConstructionScript`))