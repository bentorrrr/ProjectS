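; BP_MBug_Melee is a melee bug enemy that splits into a random number of BP_SBug_Melee bugs when it dies.
; Its Attack, noted as old mock-up mechanics, runs a short forward sphere trace for pawns while alive, sending damage and spawning a Niagara effect on hit, then signals attack end.
; Death extends the parent logic with the spawning, while block and damage responses only print debug strings.
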(event `/Game/Enemies/AI/BPI_EnemyAI.Attack`
  (bind _returnvalue (`self.K2_GetActorLocation`))
  ;[1 1 1] Old Mocking Attack Mechanics
  (if (not (`/Game/DamageSystem/BPC_DamageSystem.IsDead` (`self.BPC_DamageSystem`)))
    (bind (_outhit _returnvalue_2) (`KismetSystemLibrary.SphereTraceSingleForObjects` :`Start` _returnvalue :`End` (+ _returnvalue (* (`self.GetActorForwardVector`) 150.0)) :`Radius` 30.0 :`ObjectTypes` (`|MakeArray` "ObjectTypeQuery3" :!type "EObjectTypeQuery Enum") :`DrawDebugType` "ForDuration" :`TraceColor` (struct :`G` 0.236161 :`B` 1.0 :`A` 1.0) :`TraceHitColor` (struct :`R` 1.0 :`G` 0.739583 :`B` 0.899609 :`A` 1.0) :`DrawTime` 2.0))
    (if _returnvalue_2
      (bind (_bblockinghit _binitialoverlap _time _distance _location _impactpoint _normal _impactnormal _physmat _hitactor) (`GameplayStatics.BreakHitResult` _outhit))
      (message `/Game/DamageSystem/BPI_Damagable.TakeDamage` _hitactor (make `/Game/DamageSystem/S_DamageInfo` 10.0 "NewEnumerator1" "NewEnumerator1"))
      (`NiagaraFunctionLibrary.SpawnSystemAtLocation` "/Game/Effects/NS_EnemyHit.NS_EnemyHit" _location)
      (`self.On Attack End`)
      (else
        (`self.On Attack End`)))))

(event `self.Death`
  ;[0.05098 0.05098 0.05098] Damage Response Event
  (`parent.Death`)
  (for _ (range (+ (`KismetMathLibrary.RandomInteger` 5) 1))
    (`|SpawnActorFromClass` "/Game/Enemies/AI/EnemyClasses/BP_SBug_Melee.BP_SBug_Melee_C" (`self.GetTransform`) "AdjustIfPossibleButAlwaysSpawn" "MultiplyWithRoot" null false 4 "" 10.0 self)))

(event `self.Blocked`
  (params (CanBeParried :type Boolean))
  ;[0.05098 0.05098 0.05098] Damage Response Event
  (`KismetSystemLibrary.PrintString` "Blocked"))

(event `self.DamageResponse`
  (params (DamageResponse :type "/Game/DamageSystem/E_DamageResponse Enum" :default "NewEnumerator0"))
  ;[0.05098 0.05098 0.05098] Damage Response Event
  (`KismetSystemLibrary.PrintString` (`|GetEnumeratorNameAsString` DamageResponse)))

(fn `UserConstructionScript`
  (`parent.UserConstructionScript`))