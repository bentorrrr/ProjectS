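; Ranged bug enemy that attacks by firing pooled projectiles from its shooting position.
; Attack pulls a projectile from the object pool, ignores it in capsule movement, binds its impact event and gates refiring with a cooldown.
; Impact applies fixed damage through a damage message, reports it to AI perception and spawns a particle effect.
; Attack end is signalled both after the cooldown and on impact.
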(event `/Game/Enemies/AI/BPI_EnemyAI.Attack`
  ;[0.05127 0.05127 0.05127] Shooting Projectiles
  (if (`self.CanShoot`)
    (bind _pooledactor (`/Game/ObjectPool/AC_ObjectPooled.SpawnFromPool` (`self.AC_ObjectPooled`) (`KismetMathLibrary.MakeTransform` (.location (`SceneComponent.K2_GetComponentToWorld` (`self.ShootingPosition`))) (.rotation (`SceneComponent.K2_GetComponentToWorld` (`self.ShootingPosition`))))))
    (bind _asbp_projectiles_base (cast `/Game/DamageSystem/Projectiles/BP_ProjectilesBase` _pooledactor))
    (set `self.CanShoot` false)
    (`PrimitiveComponent.IgnoreActorWhenMoving` (`self.CapsuleComponent`) _asbp_projectiles_base true)
    (add `/Game/DamageSystem/Projectiles/BP_ProjectilesBase.OnProjectilesImpact` _asbp_projectiles_base (delegate `CustomEvent`))
    (`KismetSystemLibrary.Delay` (`self.ProjectilesCooldown`))
    (`KismetSystemLibrary.PrintString` "1")
    (set `self.CanShoot` true)
    (`/Game/Enemies/AI/BP_Enemy_Base.On Attack End`)
    (`KismetSystemLibrary.PrintString` "Hello")))

(event `CustomEvent`
  (params (OtherActor :type "Actor Object Reference") (Hit :type "HitResult Structure"))
  ;[0.05127 0.05127 0.05127] Shooting Projectiles
  (message `/Game/DamageSystem/BPI_Damagable.TakeDamage` OtherActor (make `/Game/DamageSystem/S_DamageInfo` 10.0 "NewEnumerator2" "NewEnumerator1"))
  (`AISense_Damage.ReportDamageEvent` OtherActor self 10.0 (`self.K2_GetActorLocation`))
  (`GameplayStatics.SpawnEmitterAtLocation` "/Game/Effects/NewParticleSystem.NewParticleSystem" (`.Location` (`GameplayStatics.BreakHitResult` Hit)))
  (`/Game/Enemies/AI/BP_Enemy_Base.On Attack End`))

(fn `UserConstructionScript`
  (`parent.UserConstructionScript`))