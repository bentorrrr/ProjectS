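; Melee slime enemy Blueprint whose attack is an area-of-effect explosion at its own position.
; Attack sets IsAttacking, spawns and triggers a BP_AOE_Explosion, and binds its overlap callback to apply fixed damage through a damage-info message and print the actor's name.
; Both a delay after triggering and each overlap hit lead into the shared tail that calls OnAttackEnd, then clears IsAttacking after a short delay.
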(event `/Game/Enemies/AI/BPI_EnemyAI.Attack`
  (set `self.IsAttacking` true)
  (bind _returnvalue (`|SpawnActorFromClass` "/Game/DamageSystem/AOE/BP_AOE_Explosion.BP_AOE_Explosion_C" (`self.GetTransform`) "Undefined" "MultiplyWithRoot" null true true self))
  (add `/Game/DamageSystem/AOE/BP_AOE_Base.OnAOEOverlapActor` _returnvalue (delegate `Damaging AOE Actor`))
  (`/Game/DamageSystem/AOE/BP_AOE_Base.Trigger` _returnvalue)
  (`KismetSystemLibrary.Delay` 2.0)
  (`self.On Attack End` :!label _label)
  (`KismetSystemLibrary.Delay` 0.5)
  (set `self.IsAttacking` false))

(event `Damaging AOE Actor`
  (params (Actor :type "Actor Object Reference"))
  (message `/Game/DamageSystem/BPI_Damagable.TakeDamage` Actor (make `/Game/DamageSystem/S_DamageInfo` 10.0 "NewEnumerator1" "NewEnumerator1"))
  (`KismetSystemLibrary.PrintString` (`KismetSystemLibrary.GetDisplayName` Actor))
  (goto _label))

(fn `UserConstructionScript`
  (`parent.UserConstructionScript`))