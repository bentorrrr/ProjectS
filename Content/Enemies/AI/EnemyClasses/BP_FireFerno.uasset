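; BP_FireFerno is an enemy Blueprint whose only active gameplay logic is an Attack event, noted as old mocking attack mechanics.
; Unless its damage component reports death, Attack flags it as attacking and runs a short forward sphere trace against pawns, with debug drawing.
; A hit sends a damage-info struct to the actor via a TakeDamage message and spawns a particle effect at the impact.
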(event `/Game/Enemies/AI/BPI_EnemyAI.Attack`
  (bind _returnvalue (`self.K2_GetActorLocation`))
  ;[1 1 1] Old Mocking Attack Mechanics
  (if (not (`/Game/DamageSystem/BPC_DamageSystem.IsDead` (`self.BPC_DamageSystem`)))
    (set `self.IsAttacking` true)
    (bind (_outhit _returnvalue_2) (`KismetSystemLibrary.SphereTraceSingleForObjects` :`Start` _returnvalue :`End` (+ _returnvalue (* (`self.GetActorForwardVector`) 100.0)) :`Radius` 20.0 :`ObjectTypes` (`|MakeArray` "ObjectTypeQuery3" :!type "EObjectTypeQuery Enum") :`DrawDebugType` "ForOneFrame" :`TraceColor` (struct :`G` 0.236161 :`B` 1.0 :`A` 1.0) :`TraceHitColor` (struct :`R` 1.0 :`G` 0.739583 :`B` 0.899609 :`A` 1.0) :`DrawTime` 2.0))
    (if _returnvalue_2
      (bind (_bblockinghit _binitialoverlap _time _distance _location _impactpoint _normal _impactnormal _physmat _hitactor) (`GameplayStatics.BreakHitResult` _outhit))
      (message `/Game/DamageSystem/BPI_Damagable.TakeDamage` _hitactor (make `/Game/DamageSystem/S_DamageInfo` 10.0 "NewEnumerator1" "NewEnumerator1"))
      (`GameplayStatics.SpawnEmitterAtLocation` "/Game/Effects/NewParticleSystem.NewParticleSystem" _location))))

(fn `UserConstructionScript`
  (`parent.UserConstructionScript`))