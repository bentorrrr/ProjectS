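; BP_NPC is a talkable NPC that shows its text and a dialogue widget while the main character is inside its box trigger.
; Entering the box reveals the TextRender and creates the dialogue UI, and leaving hides and removes them.
; DialogueOccurs passes NPCText to the widget, plays the matching sound and advances the row, removing the widget after the last line.
; A DoOnce guards each step and is reset immediately afterwards.
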(event `self.Box.OnComponentBeginOverlap`
  (params (OverlappedComponent :type "PrimitiveComponent Object Reference") (OtherActor :type "Actor Object Reference") (OtherComp :type "PrimitiveComponent Object Reference") (OtherBodyIndex :type Integer) (bFromSweep :type Boolean) (SweepResult :type "HitResult Structure (by ref)"))
  (cast `/Game/ThirdPerson/Blueprints/BP_MainCharacter` OtherActor)
  (`SceneComponent.SetHiddenInGame` (`self.TextRender`) false false)
  (bind _returnvalue (`|CreateWidget` "/Game/Dialouge/WB_DialogueUI.WB_DialogueUI_C"))
  (bind _output_get (set `self.DialoueUI` _returnvalue))
  (`UserWidget.AddToViewport` _output_get 0))

(event `self.Box.OnComponentEndOverlap`
  (params (OverlappedComponent :type "PrimitiveComponent Object Reference") (OtherActor :type "Actor Object Reference") (OtherComp :type "PrimitiveComponent Object Reference") (OtherBodyIndex :type Integer))
  (bind _dialoueui (`self.DialoueUI`))
  (cast `/Game/ThirdPerson/Blueprints/BP_MainCharacter` OtherActor)
  (`SceneComponent.SetHiddenInGame` (`self.TextRender`) true false)
  (`/Engine/EditorBlueprintResources/StandardMacros.IsValid` _dialoueui
    (:`Is Valid`
      (`Widget.RemoveFromParent` _dialoueui))))

(event `/Game/Dialouge/BPI_Dialogue.DialogueOccurs`
  (bind _returnvalue (+ (`/Game/Dialouge/WB_DialogueUI.TextRow` (`self.DialoueUI`)) 1))
  (`/Engine/EditorBlueprintResources/StandardMacros.DoOnce` false :!label _label
    (:`Completed`
      (set `/Game/Dialouge/WB_DialogueUI.Text` (`self.NPCText`) (`self.DialoueUI`))
      (`GameplayStatics.PlaySound2D` (`|GetArrayItem` (`self.NPCSound`) (+ (`/Game/Dialouge/WB_DialogueUI.TextRow` (`self.DialoueUI`)) 1)) 1.0 1.0 0.0 null null)
      (`Widget.SetVisibility` (`/Game/Dialouge/WB_DialogueUI.TextBlock_0` (`self.DialoueUI`)) "Visible")
      (`Widget.SetVisibility` (`/Game/Dialouge/WB_DialogueUI.Image_82` (`self.DialoueUI`)) "Visible")
      (if (> _returnvalue (- (`KismetArrayLibrary.Array_Length` (`self.NPCText`)) 1))
        (`Widget.RemoveFromParent` (`self.DialoueUI`))
        (`self.ResetDialogue`)
        (else
          (set `/Game/Dialouge/WB_DialogueUI.TextRow` _returnvalue (`self.DialoueUI`))
          (`self.ResetDialogue`))))))

(event `ResetDialogue`
  (goto _label :!via `Reset`))

(fn `UserConstructionScript`)