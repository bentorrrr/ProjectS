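; BP_PooledActor is an actor meant for object pooling that switches between in-use and idle states instead of being destroyed.
; SetInUse toggles collision, visibility and ticking together, and BeginPlay starts the actor idle.
; Entering use restarts a time-to-live timer that fires ReturnToPool, which sets the actor idle again.
; Debug prints report the state changes.
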(event `self.ReceiveBeginPlay`
  (`self.SetInUse` false))

(event `ReturnToPool`
  (`KismetSystemLibrary.PrintString` "Returning to Pool")
  (`self.SetInUse` false))

(event `SetInUse`
  (params (InUse :type Boolean))
  (`KismetSystemLibrary.PrintString` (`KismetStringLibrary.Concat_StrStr` "Set in ues is:" (`KismetStringLibrary.Conv_BoolToString` InUse)))
  (set `self.InUse` InUse)
  (`self.SetActorEnableCollision` InUse)
  (`KismetSystemLibrary.PrintString` (`KismetStringLibrary.Concat_StrStr` "Collsion is:" (`KismetStringLibrary.Conv_BoolToString` (`self.GetActorEnableCollision`))))
  (`self.SetActorHiddenInGame` (not InUse))
  (`self.SetActorTickEnabled` InUse)
  (`KismetSystemLibrary.K2_ClearAndInvalidateTimerHandle` (`self.TimeToLiveTimer`))
  (if InUse
    (bind _returnvalue (`KismetSystemLibrary.K2_SetTimerDelegate` (delegate `ReturnToPool`) (`self.TimeToLive`)))
    (set `self.TimeToLiveTimer` _returnvalue)))

(fn `UserConstructionScript`)