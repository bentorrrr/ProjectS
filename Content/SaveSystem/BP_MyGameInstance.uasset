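; Game instance that owns the player's save data, keeping it in memory for the session and persisting it to a single save slot.
; On Init it loads the existing BP_SaveData_Player from the slot, or creates a new save object if none exists.
; SavePlayerData copies inventory data into that object and writes it to disk, while GetSaveData returns it wrapped in a save-data struct.
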(event `self.ReceiveInit`
  (`self.LoadGameData`))

(event `/Game/SaveSystem/BPI_SaveSystem.LoadGameData`
  ;[1 1 1] Load Game Data
  (bind _returnvalue (`GameplayStatics.DoesSaveGameExist` "slot1"))
  (if _returnvalue
    (bind _returnvalue_2 (`GameplayStatics.LoadGameFromSlot` "slot1"))
    (bind _asbp_save_data_player (cast `/Game/SaveSystem/BP_SaveData_Player` _returnvalue_2))
    (set `self.SaveDataPlayer` _asbp_save_data_player)
    (else
      (bind _returnvalue_3 (`GameplayStatics.CreateSaveGameObject` "/Game/SaveSystem/BP_SaveData_Player.BP_SaveData_Player_C"))
      (set `self.SaveDataPlayer` _returnvalue_3))))

(event `/Game/SaveSystem/BPI_SaveSystem.SaveGameData`
  ;[1 1 1] Save Game Data
  (`GameplayStatics.SaveGameToSlot` (`self.SaveDataPlayer`) "slot1"))

(event `/Game/SaveSystem/BPI_SaveSystem.SavePlayerData`
  (params (InventoryData :type "Array of /Game/InventorySystem/ItemData/S_ItemSlot Structure (by ref)"))
  ;[1 1 1] Save Player Data
  (set `/Game/SaveSystem/BP_SaveData_Player.InventoryData` InventoryData (`self.SaveDataPlayer`))
  (`/Game/SaveSystem/BPI_SaveSystem.SaveGameData`))

(fn `GetSaveData`
  (returns (SaveData :type "/Game/SaveSystem/Structs/S_SaveData Structure"))
  ;[1 1 1] Get Save Data
  (return (make `/Game/SaveSystem/Structs/S_SaveData` (`self.SaveDataPlayer`))))