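; Blueprint library of save helpers for player inventory, level container data and a "Game Saved" sound with debug print.
; SavePlayerData sends the main character's inventory data to the Game Instance through a message call.
; SaveLevelData clears the Game Mode's container arrays and those returned by each BP_Container_Base actor, then messages the Game Mode with its ContainerData.
; No container entries are re-added before that message.
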(fn `SaveLevelData`
  (bind _asbp_third_person_game_mode (cast `/Game/ThirdPerson/Blueprints/BP_ThirdPersonGameMode` (`GameplayStatics.GetGameMode` null)))
  (bind _containerdata (`/Game/SaveSystem/BP_SaveData_Level.ContainerData` (`/Game/ThirdPerson/Blueprints/BP_ThirdPersonGameMode.SaveDataLevel` _asbp_third_person_game_mode)))
  (bind (_containers _containerinventories) (break `/Game/SaveSystem/Structs/S_ContainerData` _containerdata))
  (`KismetArrayLibrary.Array_Clear` _containers)
  (`KismetArrayLibrary.Array_Clear` _containerinventories)
  (bind _outactors (`GameplayStatics.GetAllActorsOfClass` null "/Game/InventorySystem/Container/BP_Container_Base.BP_Container_Base_C"))
  (for _array_element _outactors
    (bind _containerdata_2 (`/Game/InventorySystem/Container/BP_Container_Base.GetContainerData` _array_element))
    (bind (_containers_2 _containerinventories_2) (break `/Game/SaveSystem/Structs/S_ContainerData` _containerdata_2))
    (`KismetArrayLibrary.Array_Clear` _containers_2)
    (`KismetArrayLibrary.Array_Clear` _containerinventories_2))
  (message `/Game/SaveSystem/BPI_SaveSystem.SaveLevelData` (`GameplayStatics.GetGameMode` null) _containerdata))

(fn `SavePlayerData`
  (bind _asbp_main_character (cast `/Game/ThirdPerson/Blueprints/BP_MainCharacter` (`GameplayStatics.GetPlayerCharacter` null)))
  (message `/Game/SaveSystem/BPI_SaveSystem.SavePlayerData` (`GameplayStatics.GetGameInstance` null) (`/Game/InventorySystem/BPC_Inventory.GetInventoryData` (`/Game/ThirdPerson/Blueprints/BP_MainCharacter.BPC_Inventory` _asbp_main_character))))

(fn `SaveSFX`
  (`GameplayStatics.PlaySound2D` null null 1.0 1.0 0.0 null null)
  (`KismetSystemLibrary.PrintString` null "Game Saved"))