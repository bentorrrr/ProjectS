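; BP_LocationDialogue is a trigger actor that starts a location-based dialogue when the main character enters its box.
; On overlap it scans the player's quest log for quest 008 at stage 0 or 1, debug-printing each check.
; A match opens WB_Dialogue with quest 002, stage 99, disables character input and switches to UI-only input with a cursor.
; It has no one-shot guard, so re-entry can retrigger it.
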(event `self.TriggerBox.OnComponentBeginOverlap`
  (params (OverlappedComponent :type "PrimitiveComponent Object Reference") (OtherActor :type "Actor Object Reference") (OtherComp :type "PrimitiveComponent Object Reference") (OtherBodyIndex :type Integer) (bFromSweep :type Boolean) (SweepResult :type "HitResult Structure (by ref)"))
  (bind _returnvalue (`GameplayStatics.GetPlayerController` 0))
  (bind _wb_dialogue (`self.WB_Dialogue`))
  (bind _ac_questlog (`/Game/ThirdPerson/Blueprints/BP_MainCharacter.AC_QuestLog` (`/Game/QuestSystem/Interaction/BPFL_CommonFunction.GetMainPlayerCharacter`)))
  (cast `/Game/ThirdPerson/Blueprints/BP_MainCharacter` OtherActor)
  (for _array_element (`/Game/QuestSystem/AC_QuestLog.CurrentQuests` _ac_questlog)
    (bind _questid (`/Game/QuestSystem/BP_QuestBase.QuestID` _array_element))
    (bind _questactor (`/Game/QuestSystem/AC_QuestLog.GetQuestActor` _ac_questlog _questid))
    (bind _currentstage (`/Game/QuestSystem/BP_QuestBase.CurrentStage` _questactor))
    (bind _returnvalue_2 (or (and (== _questid "008") (== _currentstage 1)) (and (== _questid "008") (== _currentstage 0))))
    (`KismetSystemLibrary.PrintString` (`KismetStringLibrary.Conv_BoolToString` _returnvalue_2) true true (struct :`G` 0.078744 :`B` 1.0 :`A` 1.0))
    (if _returnvalue_2
      (bind _returnvalue_3 (`|CreateWidget` "/Game/NewDialogue/WB_Dialogue.WB_Dialogue_C" _returnvalue))
      (set `self.WB_Dialogue` _returnvalue_3)
      (`UserWidget.AddToViewport` _wb_dialogue 0)
      (`/Game/NewDialogue/WB_Dialogue.StartDialogue` _wb_dialogue "002" 99)
      (`self.DisableInput` (`GameplayStatics.GetPlayerCharacter` 0) (`GameplayStatics.GetPlayerController` 0))
      (`WidgetBlueprintLibrary.SetInputMode_UIOnlyEx` _returnvalue _wb_dialogue)
      (set `PlayerController.bShowMouseCursor` true _returnvalue))))

(fn `UserConstructionScript`)