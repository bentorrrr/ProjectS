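; Location trigger actor that opens quest dialogue when its trigger box is overlapped, based on the main player's quest log.
; If quest 008 is completed and IsOpen is set, it starts a special quest 010 dialogue once, clearing IsOpen.
; Otherwise, for the main character, it debug-prints and checks current quests for specific 009 or 010 stages, starting matching dialogue.
; Both paths create the dialogue widget, disable player input and switch to UI-only mouse control.
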(event `self.TriggerBox.OnComponentBeginOverlap`
  (params (OverlappedComponent :type "PrimitiveComponent Object Reference") (OtherActor :type "Actor Object Reference") (OtherComp :type "PrimitiveComponent Object Reference") (OtherBodyIndex :type Integer) (bFromSweep :type Boolean) (SweepResult :type "HitResult Structure (by ref)"))
  (bind _returnvalue (`GameplayStatics.GetPlayerController` 0))
  (bind _returnvalue_2 (`GameplayStatics.GetPlayerController` 0))
  (bind _wb_dialogue (`self.WB_Dialogue`))
  (bind _wb_dialogue_2 (`self.WB_Dialogue`))
  (bind _ac_questlog (`/Game/ThirdPerson/Blueprints/BP_MainCharacter.AC_QuestLog` (`/Game/QuestSystem/Interaction/BPFL_CommonFunction.GetMainPlayerCharacter`)))
  (if (and (`KismetArrayLibrary.Array_Contains` (`/Game/QuestSystem/AC_QuestLog.CompletedQuest` (`/Game/ThirdPerson/Blueprints/BP_MainCharacter.AC_QuestLog` (`/Game/QuestSystem/Interaction/BPFL_CommonFunction.GetMainPlayerCharacter`))) "008") (`self.IsOpen`))
    (bind _returnvalue_3 (`|CreateWidget` "/Game/NewDialogue/WB_Dialogue.WB_Dialogue_C" _returnvalue))
    (set `self.WB_Dialogue` _returnvalue_3)
    (`UserWidget.AddToViewport` _wb_dialogue_2 0)
    (`/Game/NewDialogue/WB_Dialogue.StartDialogue` _wb_dialogue_2 "010" 99)
    (`self.DisableInput` (`GameplayStatics.GetPlayerCharacter` 0) (`GameplayStatics.GetPlayerController` 0))
    (`WidgetBlueprintLibrary.SetInputMode_UIOnlyEx` _returnvalue _wb_dialogue_2)
    (set `PlayerController.bShowMouseCursor` true _returnvalue)
    (set `self.IsOpen` false)
    (else
      (cast `/Game/ThirdPerson/Blueprints/BP_MainCharacter` OtherActor)
      (for _array_element (`/Game/QuestSystem/AC_QuestLog.CurrentQuests` _ac_questlog)
        (bind _questid (`/Game/QuestSystem/BP_QuestBase.QuestID` _array_element))
        (bind _questactor (`/Game/QuestSystem/AC_QuestLog.GetQuestActor` _ac_questlog _questid))
        (bind _currentstage (`/Game/QuestSystem/BP_QuestBase.CurrentStage` _questactor))
        (bind _returnvalue_4 (or (and (== _questid "009") (== _currentstage 1)) (and (== _questid "010") (== _currentstage 0))))
        (`KismetSystemLibrary.PrintString` (`KismetStringLibrary.Conv_BoolToString` _returnvalue_4) true true (struct :`G` 0.004941 :`B` 1.0 :`A` 1.0))
        (if _returnvalue_4
          (bind _returnvalue_5 (`|CreateWidget` "/Game/NewDialogue/WB_Dialogue.WB_Dialogue_C" _returnvalue_2))
          (set `self.WB_Dialogue` _returnvalue_5)
          (`UserWidget.AddToViewport` _wb_dialogue 0)
          (`/Game/NewDialogue/WB_Dialogue.StartDialogue` _wb_dialogue _questid _currentstage)
          (`self.DisableInput` (`GameplayStatics.GetPlayerCharacter` 0) (`GameplayStatics.GetPlayerController` 0))
          (`WidgetBlueprintLibrary.SetInputMode_UIOnlyEx` _returnvalue_2 _wb_dialogue)
          (set `PlayerController.bShowMouseCursor` true _returnvalue_2))))))

(fn `UserConstructionScript`)