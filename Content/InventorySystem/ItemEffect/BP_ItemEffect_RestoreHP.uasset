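; BP_ItemEffect_RestoreHP is an inventory item effect actor that restores a fixed amount of health to the main player.
; The heal fires once on BeginPlay, so spawning the actor is what applies the effect, and nothing here destroys it afterwards.
; Its own TakeDamage, Heal and health getter functions are empty stubs returning false or zero.
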(event `self.ReceiveBeginPlay`
  (`/Game/DamageSystem/BPI_Damagable.Heal` (`/Game/QuestSystem/Interaction/BPFL_CommonFunction.GetMainPlayerCharacter`) 20.0))

(fn `Get Current Health`
  (returns (Health :type "Float (double-precision)"))
  (return 0.0))

(fn `GetMaxHealth`
  (returns (MaxHealth :type "Float (double-precision)"))
  (return 0.0))

(fn `Heal`
  (params (HealAmount :type "Float (double-precision)" :default 0.0))
  (returns (NewHealth :type "Float (double-precision)"))
  (return 0.0))

(fn `TakeDamage`
  (params (DamageInfo :type "/Game/DamageSystem/S_DamageInfo Structure"))
  (returns (WasDamaged :type Boolean))
  (return false))

(fn `UserConstructionScript`
  (`parent.UserConstructionScript`))