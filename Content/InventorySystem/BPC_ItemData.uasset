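; Actor component that turns its owner into an inventory pickup, holding an item row ID and quantity.
; Interact passes both to the interactor's inventory component, if valid, through Pickup.
; On success it looks up the row in DT_ItemData and, if found, plays that item's pickup sound at the owner's location and destroys the owner.
; OnInteract is empty and FocusTarget returns an empty string.
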(event `/Game/InventorySystem/BPI_Interact.Interact`
  (params (Interactor :type "/Game/ThirdPerson/Blueprints/BP_MainCharacter Object Reference"))
  (bind _bpc_inventory (`/Game/ThirdPerson/Blueprints/BP_MainCharacter.BPC_Inventory` Interactor)
    (:`then`
      (bind _success (`/Game/InventorySystem/BPC_Inventory.Pickup` _bpc_inventory (`.RowName` (break `DataTableRowHandle` (`self.ItemID`))) (`self.ItemQuantity`)))
      (if _success
        (bind _returnvalue (`|GetDataTableRow` "/Game/InventorySystem/ItemData/DT_ItemData.DT_ItemData" (`.RowName` (break `DataTableRowHandle` (`self.ItemID`))))
          (:`then`
            (`GameplayStatics.PlaySoundAtLocation` (`.PickUp_5_51FE6E0447AFFFE94685F0B93F061194` (break `/Game/InventorySystem/ItemData/S_ItemSFX` (`.SFX_23_E69ADC484634F87B1A0EA295E3DA04FB` (break `/Game/InventorySystem/ItemData/S_ItemData` _returnvalue)))) (`Actor.K2_GetActorLocation` (`self.GetOwner`)) (struct) 1.0 1.0 0.0 null null null null)
            (`Actor.K2_DestroyActor` (`self.GetOwner`))))))
    (:`else`)))

(event `/Game/InventorySystem/BPI_Interact.OnInteract`)

(fn `FocusTarget`
  (returns (Message :type Text))
  (return ""))