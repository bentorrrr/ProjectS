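; Chest container actor for the inventory system that opens and closes its lid.
; OnInteract and UpdateContainer share one toggle that flips IsOpen and plays the matching open or close sound at the chest's location.
; A timeline plays forward or in reverse, its track interpolating SecondMesh's relative roll to swing the lid.
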(event `/Game/InventorySystem/BPI_Interact.OnInteract`
  (bind _returnvalue (`self.K2_GetActorLocation`))
  (bind (_open _close) (break `/Game/Sound/SFX_Chest/S_ContainerSFX` (`self.ContainerSFX`)))
  (if (not (`self.IsOpen`)) :!label _label
    (set `self.IsOpen` true)
    (`GameplayStatics.PlaySoundAtLocation` _open _returnvalue (struct) 1.0 1.0 0.0 null null null null)
    (bind (_direction _containertrack) (`Timeline|ContainerTimeline` :!label _label_2)
      (:`Update`
        (`SceneComponent.K2_SetRelativeRotation` (`self.SecondMesh`) (`KismetMathLibrary.MakeRotator` (`KismetMathLibrary.Lerp` 0.0 -120.0 _containertrack)) false false)))
    (else
      (set `self.IsOpen` false)
      (`GameplayStatics.PlaySoundAtLocation` _close _returnvalue (struct) 1.0 1.0 0.0 null null null null)
      (goto _label_2 :!via `Reverse`))))

(event `self.UpdateContainer`
  (goto _label))

(fn `UserConstructionScript`
  (`parent.UserConstructionScript`))