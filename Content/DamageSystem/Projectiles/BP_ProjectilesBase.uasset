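; Base pooled projectile that flies at a target and broadcasts its impacts.
; On activation it ignores its instigator or owner, then sets velocity toward the target, or from player 0's pawn rotation without one; deactivation zeroes it.
; Box hits, or overlaps with "Collidable"-tagged actors, fire the impact event, spawn effect and sound, then return it to the pool.
; The construction script applies speed, gravity and optional homing on a valid target.
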(event `self.SetInUse`
  (params (InUse :type Boolean))
  (bind _returnvalue (`self.GetInstigator`))
  (`parent.SetInUse` InUse)
  (if InUse
    (`PrimitiveComponent.IgnoreActorWhenMoving` (`self.BoxCollision`) (select `bool` (`KismetSystemLibrary.IsValid` _returnvalue) :`false` (`self.GetOwner`) :`true` _returnvalue :!type "Actor Object Reference") true)
    (`self.Target`
      (:`then`
        (`KismetSystemLibrary.PrintString` "Valid")
        (`self.RotateToTarget`))
      (:`else`
        (set `MovementComponent.Velocity` (* (`self.Speed`) (`self.K2_GetActorRotation` (`GameplayStatics.GetPlayerPawn` 0))) (`self.ProjectileMovement`))))
    (else
      (set `MovementComponent.Velocity` (0.0 0.0 0.0) (`self.ProjectileMovement`)))))

(event `RotateToTarget`
  ;[1 1 1] Rotate to Actor Location
  (bind _output_get (set `MovementComponent.Velocity` (* (`KismetMathLibrary.GetDirectionUnitVector` (`self.K2_GetActorLocation`) (`self.K2_GetActorLocation` (`self.Target`))) (`self.Speed`)) (`self.ProjectileMovement`)))
  (`KismetSystemLibrary.PrintString` (`KismetStringLibrary.Conv_VectorToString` _output_get)))

(event `self.BoxCollision.OnComponentHit`
  (params (HitComponent :type "PrimitiveComponent Object Reference") (OtherActor :type "Actor Object Reference") (OtherComp :type "PrimitiveComponent Object Reference") (NormalImpulse :type "Vector Structure") (Hit :type "HitResult Structure (by ref)"))
  (bind (_bblockinghit _binitialoverlap _time _distance _location) (`GameplayStatics.BreakHitResult` Hit))
  ;[1 1 1] On Impact
  (`self.OnProjectilesImpact` OtherActor Hit)
  (`NiagaraFunctionLibrary.SpawnSystemAtLocation` (`self.Impact Effect`) _location)
  (`GameplayStatics.PlaySoundAtLocation` (`self.Impact Sound`) _location (struct) 1.0 1.0 0.0 null null null null)
  (`self.ReturnToPool`))

(event `self.ReceiveActorBeginOverlap`
  (params (OtherActor :type "Actor Object Reference"))
  (bind _returnvalue (`self.K2_GetActorLocation`))
  (if (`self.ActorHasTag` OtherActor "Collidable")
    (`KismetSystemLibrary.PrintString` "Collided")
    (`self.OnProjectilesImpact` OtherActor (`GameplayStatics.MakeHitResult` false false 0.0 0.0 (0.0 0.0 0.0) (0.0 0.0 0.0) (0.0 0.0 1.0) (0.0 0.0 1.0) null OtherActor))
    (`NiagaraFunctionLibrary.SpawnSystemAtLocation` (`self.Impact Effect`) _returnvalue)
    (`GameplayStatics.PlaySoundAtLocation` (`self.Impact Sound`) _returnvalue (struct) 1.0 1.0 0.0 null null null null)
    (`self.ReturnToPool`)))

(fn `UserConstructionScript`
  (bind _projectilemovement (`self.ProjectileMovement`))
  (bind _speed (`self.Speed`))
  (set `ProjectileMovementComponent.InitialSpeed` _speed _projectilemovement)
  (set `ProjectileMovementComponent.MaxSpeed` _speed _projectilemovement)
  (set `ProjectileMovementComponent.ProjectileGravityScale` (`self.Gravity`) _projectilemovement)
  (`self.Target`
    (:`then`
      (if (`self.IsHoming`)
        (set `ProjectileMovementComponent.bIsHomingProjectile` true _projectilemovement)
        (set `ProjectileMovementComponent.HomingTargetComponent` (`Actor.RootComponent` (`self.Target`)) _projectilemovement)))
    (:`else`)))