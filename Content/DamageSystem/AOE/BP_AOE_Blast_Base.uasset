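; BP_AOE_Blast_Base is a base Blueprint for blast area-of-effect actors in the damage system, adding effects and sound to its parent's AOE sphere.
; SpawnAOESphere runs the parent logic, then spawns BlastEffect as an attached Niagara system and plays Sound at the actor's location.
; The actor destroys itself when the effect finishes, or after a short delay if no valid effect is set.
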(event `self.SpawnAOESphere`
  (`parent.SpawnAOESphere`)
  (`self.SpawnBlastEffect`)
  (`self.PlayBlastSound`))

(event `SpawnBlastEffect`
  ;[1 1 1] Spawn BlastEffects
  (bind _blasteffect (`self.BlastEffect`)
    (:`then`
      (bind _returnvalue (`NiagaraFunctionLibrary.SpawnSystemAttached` _blasteffect (`self.DefaultSceneRoot`) "None" (0.0 0.0 0.0) (struct) "KeepRelativeOffset"))
      (add `NiagaraComponent.OnSystemFinished` _returnvalue (delegate `SystemFinished`)))
    (:`else`
      (`KismetSystemLibrary.Delay` 1.0)
      (`self.K2_DestroyActor`))))

(event `SystemFinished`
  (params (PSystem :type "NiagaraComponent Object Reference"))
  ;[1 1 1] Spawn BlastEffects
  (`self.K2_DestroyActor`))

(event `PlayBlastSound`
  ;[1 1 1] Play Blast Sound
  (bind _sound (`self.Sound`)
    (:`then`
      (`GameplayStatics.PlaySoundAtLocation` _sound (`self.K2_GetActorLocation`) (struct) 1.0 1.0 0.0 null null null null))
    (:`else`)))

(fn `UserConstructionScript`
  (`parent.UserConstructionScript`))