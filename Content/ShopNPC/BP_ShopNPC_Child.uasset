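; BP_ShopNPC_Child is a child Blueprint for a shop NPC that toggles between open and closed states with sound feedback.
; OnInteract and UpdateNPC share one branch that flips IsOpen and plays the matching NPCSFX open or close sound at the actor's location.
; BeginPlay is a disabled stub, and the construction script only calls the parent.
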(event `/Game/InventorySystem/BPI_Interact.OnInteract`
  (bind _returnvalue (`self.K2_GetActorLocation`))
  (bind (_open _close) (break `/Game/Sound/SFX_Chest/S_ContainerSFX` (`self.NPCSFX`)))
  (if (not (`self.IsOpen`)) :!label _label
    (set `self.IsOpen` true)
    (`GameplayStatics.PlaySoundAtLocation` _open _returnvalue (struct) 1.0 1.0 0.0 null null null null)
    (else
      (set `self.IsOpen` false)
      (`GameplayStatics.PlaySoundAtLocation` _close _returnvalue (struct) 1.0 1.0 0.0 null null null null))))

(event `self.UpdateNPC`
  (goto _label))

(fn `UserConstructionScript`
  (`parent.UserConstructionScript`))