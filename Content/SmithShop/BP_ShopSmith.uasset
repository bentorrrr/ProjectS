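; Interactable blacksmith shop with a saveable inventory that runs a timed weapon-order minigame.
; Interact swaps gameplay for shop UI and audio, then offers random orders from DT_OrderData.
; Accepting an order enables crafting buttons and starts a Tick countdown; expiry docks shop time and reschedules the session timer, while declining rerolls.
; Session end clears items and UI, restores player control and minimap, and advances the GameInstance time slot.
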(event `UpdateContainer`)

(event `self.ReceiveBeginPlay`
  (bind _bpc_inventory (`self.BPC_Inventory`))
  (`KismetSystemLibrary.Delay` 0.2)
  (bind _asbp_third_person_game_mode (cast `/Game/ThirdPerson/Blueprints/BP_ThirdPersonGameMode` (`GameplayStatics.GetGameMode`)))
  (bind _returnvalue (`GameplayStatics.DoesSaveGameExist` (`/Game/ThirdPerson/Blueprints/BP_ThirdPersonGameMode.LevelData` _asbp_third_person_game_mode)))
  (if _returnvalue
    (bind _savedata (message `/Game/SaveSystem/BPI_SaveSystem.GetSaveData` (`GameplayStatics.GetGameMode`)))
    (bind (_playerdata _leveldata) (break `/Game/SaveSystem/Structs/S_SaveData` _savedata))
    (`/Engine/EditorBlueprintResources/StandardMacros.IsValid` _leveldata
      (:`Is Valid`
        (`self.LoadContainerData` (`/Game/SaveSystem/BP_SaveData_Level.ContainerData` _leveldata))
        (`self.EnableInput` (`GameplayStatics.GetPlayerController` 0))))
    (else
      (set `/Game/InventorySystem/BPC_Inventory.ItemSlots` (`self.ContainerContent`) _bpc_inventory)
      (`KismetArrayLibrary.Array_Resize` (`/Game/InventorySystem/BPC_Inventory.ItemSlots` _bpc_inventory) (`self.ContainerSize`)))))

(event `self.OnInteract`)

(event `TriggerNewOrder`
  (bind _orderdetailwidget (`self.OrderDetailWidget`))
  (if (> (`self.ShopTime`) 0.0)
    (`/Engine/EditorBlueprintResources/StandardMacros.IsValid` _orderdetailwidget
      (:`Is Valid`
        (`Widget.RemoveFromParent` _orderdetailwidget)
        (`self.SpawnNewOrderWidget `)
        (`Widget.SetIsEnabled` (`/Game/SmithShop/UI/WB_SlotandInventoryDisplay.CraftBtn` (`self.SlotAndInventory`)) false)
        (`Widget.SetIsEnabled` (`/Game/SmithShop/UI/WB_SlotandInventoryDisplay.swordBtn` (`self.SlotAndInventory`)) false)
        (`Widget.SetIsEnabled` (`/Game/SmithShop/UI/WB_SlotandInventoryDisplay.bowBtn` (`self.SlotAndInventory`)) false)
        (`Widget.SetIsEnabled` (`/Game/SmithShop/UI/WB_SlotandInventoryDisplay.staffBtn` (`self.SlotAndInventory`)) false)))))

(event `self.Box.OnComponentBeginOverlap`
  (params (OverlappedComponent :type "PrimitiveComponent Object Reference") (OtherActor :type "Actor Object Reference") (OtherComp :type "PrimitiveComponent Object Reference") (OtherBodyIndex :type Integer) (bFromSweep :type Boolean) (SweepResult :type "HitResult Structure (by ref)"))
  (cast `/Game/ThirdPerson/Blueprints/BP_MainCharacter` OtherActor)
  (set `self.IsPlayerInRange	` true))

(event `self.Box.OnComponentEndOverlap`
  (params (OverlappedComponent :type "PrimitiveComponent Object Reference") (OtherActor :type "Actor Object Reference") (OtherComp :type "PrimitiveComponent Object Reference") (OtherBodyIndex :type Integer))
  (cast `/Game/ThirdPerson/Blueprints/BP_MainCharacter` OtherActor)
  (set `self.IsPlayerInRange	` false))

(event `self.Interact`
  (params (Interactor :type "/Game/ThirdPerson/Blueprints/BP_MainCharacter Object Reference"))
  (bind _returnvalue (`GameplayStatics.GetPlayerController` 0))
  (bind _minimap (`self.Minimap`))
  (set `self.IsBGMClose` true)
  (set `self.IsShopClose` false)
  (`self.DisableInput` (`GameplayStatics.GetPlayerCharacter` 0) (`GameplayStatics.GetPlayerController` 0))
  (`GameplayStatics.PlaySound2D` "/Game/SmithShop/UI/soundElement/big-bell-330719.big-bell-330719" 1.0 1.0 0.0 null null)
  (bind _returnvalue_2 (`|CreateWidget` "/Game/SmithShop/UI/WB_OpenShop.WB_OpenShop_C"))
  (`UserWidget.AddToViewport` _returnvalue_2 0)
  (`KismetSystemLibrary.Delay` 2.0)
  (bind _returnvalue_3 (`|CreateWidget` "/Game/Menu/WB_Fade.WB_Fade_C"))
  (`UserWidget.AddToViewport` _returnvalue_3 0)
  (`/Game/Menu/WB_Fade.PlayFadeIn` _returnvalue_3)
  (`KismetSystemLibrary.Delay` 2.0)
  (bind _returnvalue_4 (`GameplayStatics.SpawnSound2D` "/Game/SmithShop/UI/soundElement/blacksmithBGM.blacksmithBGM" 0.1 1.0 0.0 null false false))
  (set `self.blacksmithsound` _returnvalue_4)
  (bind _returnvalue_5 (`GameplayStatics.SpawnSound2D` "/Game/SmithShop/UI/soundElement/shopBGM.shopBGM" 0.2 1.0 0.0 null false false))
  (set `self.bgshop` _returnvalue_5)
  (bind _returnvalue_6 (`GameplayStatics.SpawnSound2D` "/Game/ThirdPerson/Maps/BGM/aspose_audio_compress_133908570942870002.aspose_audio_compress_133908570942870002" 0.1 1.0 0.0 null false false))
  (set `self.ambientshop` _returnvalue_6)
  (bind _asbp_mycontroller (cast `/Game/ThirdPerson/Blueprints/BP_Mycontroller` (`GameplayStatics.GetPlayerController` 0)))
  (bind _returnvalue_7 (`/Game/ThirdPerson/UI/WB_PlayerHUD.CreateSlotShop` (`/Game/ThirdPerson/Blueprints/BP_Mycontroller.WB_PlayerHUD` _asbp_mycontroller) (`self.BPC_Inventory`)))
  (set `self.SlotAndInventory` _returnvalue_7)
  (if (not (`self.IsShopOpen`))
    (set `self.IsShopOpen` true)
    (bind _foundwidgets (`WidgetBlueprintLibrary.GetAllWidgetsOfClass` "/Game/MapSystem/WB_MiniMap.WB_MiniMap_C" false))
    (`Widget.RemoveFromParent` (`|GetArrayItem` _foundwidgets))
    (`/Engine/EditorBlueprintResources/StandardMacros.IsValid` _minimap
      (:`Is Valid`
        (`Widget.RemoveFromParent` _minimap)
        (set `self.Minimap` (`self.Minimap_0`)))
      (:`Is Not Valid`
        _))
    (bind _returnvalue_8 (`KismetSystemLibrary.K2_SetTimerDelegate` (delegate `EndShopSessioNew`) 60.0))
    (set `self.ShopTimerHandle	` _returnvalue_8)
    (bind _returnvalue_9 (`|CreateWidget` "/Game/SmithShop/UI/WB_BG.WB_BG_C" (`GameplayStatics.GetPlayerController` 0)))
    (bind _output_get (set `self.BG` _returnvalue_9))
    (`UserWidget.AddToViewport` _output_get 0)
    (bind _returnvalue_10 (`|CreateWidget` "/Game/SmithShop/UI/WB_TimerShop.WB_TimerShop_C" (`GameplayStatics.GetPlayerController` 0)))
    (bind _output_get_2 (set `self.ShopTimerWidgetInstance` _returnvalue_10))
    (`UserWidget.AddToViewport` _output_get_2 1)
    (set `/Game/SmithShop/UI/WB_TimerShop.RemainingTime` (`self.ShopTime`) (`self.ShopTimerWidgetInstance`))
    (bind _returnvalue_11 (`|CreateWidget` "/Game/SmithShop/UI/WB_OrderDetail.WB_OrderDetail_C" (`GameplayStatics.GetPlayerController` 0) null))
    (bind _output_get_3 (set `self.OrderDetailWidget` _returnvalue_11))
    (`UserWidget.AddToViewport` _output_get_3 1)
    (set `PlayerController.bShowMouseCursor` true _returnvalue)
    (`WidgetBlueprintLibrary.SetInputMode_UIOnlyEx` _returnvalue (`self.OrderDetailWidget`))
    (add `/Game/SmithShop/UI/WB_OrderDetail.OnOrderAccepted` _output_get_3 (delegate `HandleOrderAccepted`))
    (add `/Game/SmithShop/UI/WB_OrderDetail.OnOrderDeclined` _output_get_3 (delegate `HandleOrderDeclined`))
    (bind _newparam (`self.GetRandomOrder` (`self.CurrentOrder`)))
    (bind _output_get_4 (set `self.CurrentOrder` _newparam))
    (`/Game/SmithShop/UI/WB_OrderDetail.UpdateUI` _output_get_3 _output_get_4)
    (`Widget.SetIsEnabled` (`/Game/SmithShop/UI/WB_SlotandInventoryDisplay.CraftBtn` (`self.SlotAndInventory`)) false)
    (`Widget.SetIsEnabled` (`/Game/SmithShop/UI/WB_SlotandInventoryDisplay.swordBtn` (`self.SlotAndInventory`)) false)
    (`Widget.SetIsEnabled` (`/Game/SmithShop/UI/WB_SlotandInventoryDisplay.bowBtn` (`self.SlotAndInventory`)) false)
    (`Widget.SetIsEnabled` (`/Game/SmithShop/UI/WB_SlotandInventoryDisplay.staffBtn` (`self.SlotAndInventory`)) false)))

(event `EndShopSessioNew`
  (bind _returnvalue (`GameplayStatics.GetPlayerController` 0))
  (`GameplayStatics.PlaySound2D` "/Game/SmithShop/UI/soundElement/big-bell-330719.big-bell-330719" 1.0 1.0 0.0 null null)
  (`AudioComponent.FadeOut` (`self.bgshop`) 0.2 0.0 "Linear")
  (`AudioComponent.FadeOut` (`self.ambientshop`) 0.2 0.0 "Linear")
  (`AudioComponent.FadeOut` (`self.blacksmithsound`) 0.2 0.0 "Linear")
  (bind _returnvalue_2 (`|CreateWidget` "/Game/SmithShop/UI/WB_CloseShop.WB_CloseShop_C"))
  (`UserWidget.AddToViewport` _returnvalue_2 3)
  (`KismetSystemLibrary.Delay` 2.0)
  (bind _returnvalue_3 (`|CreateWidget` "/Game/Menu/WB_Fade.WB_Fade_C"))
  (`UserWidget.AddToViewport` _returnvalue_3 4)
  (`/Game/Menu/WB_Fade.PlayFadeIn` _returnvalue_3)
  (`KismetSystemLibrary.Delay` 2.0)
  (`/Game/SmithShop/UI/WB_SlotandInventoryDisplay.RemoveAllItem` :`self` (`self.SlotAndInventory`))
  (`Widget.RemoveFromParent` (`self.ShopTimerWidgetInstance`))
  (`Widget.RemoveFromParent` (`self.OrderDetailWidget`))
  (`/Game/SmithShop/UI/WB_SlotandInventoryDisplay.RemoveAllItem` (`self.SlotAndInventory`) (`/Game/InventorySystem/BPC_Inventory.ItemSlots` (`self.Container Inventory`)))
  (bind _asbp_mycontroller (cast `/Game/ThirdPerson/Blueprints/BP_Mycontroller` (`GameplayStatics.GetPlayerController` 0)))
  (`/Game/ThirdPerson/UI/WB_PlayerHUD.DeleteSlotShop` (`/Game/ThirdPerson/Blueprints/BP_Mycontroller.WB_PlayerHUD` _asbp_mycontroller))
  (`Widget.RemoveFromParent` (`self.BG`))
  (`Widget.RemoveFromParent` (`/Game/SmithShop/UI/WB_SlotandInventoryDisplay.weaponBook` (`self.SlotAndInventory`)))
  (set `self.IsShopOpen` false)
  (set `PlayerController.bShowMouseCursor` false _returnvalue)
  (`WidgetBlueprintLibrary.SetInputMode_GameOnly` _returnvalue)
  (bind _returnvalue_4 (`|CreateWidget` "/Game/MapSystem/WB_MiniMap.WB_MiniMap_C" (`GameplayStatics.GetPlayerController` 0)))
  (bind _output_get (set `self.Minimap` _returnvalue_4))
  (`UserWidget.AddToViewport` _output_get 0)
  (`self.EnableInput` (`GameplayStatics.GetPlayerCharacter` 0) _returnvalue)
  (set `self.ShopTime` 300.0)
  (bind _asbp_main_game_instance (cast `/Game/Utils/BP_MainGameInstance` (`GameplayStatics.GetGameInstance`)))
  (`/Game/Utils/BP_MainGameInstance.AdvanceTimeSlot` _asbp_main_game_instance))

(event `HandleOrderDeclined`
  (bind _orderdetailwidget (`self.OrderDetailWidget`))
  (if (> (`self.ShopTime`) 0.0)
    (`/Engine/EditorBlueprintResources/StandardMacros.IsValid` _orderdetailwidget
      (:`Is Valid`
        (`Widget.RemoveFromParent` _orderdetailwidget)
        (`self.SpawnNewOrderWidget `)))))

(event `HandleOrderAccepted`
  (bind _orderdetailwidget (`self.OrderDetailWidget`))
  (bind (_currentorder_adventureimage _currentorder_weapontype _currentorder_monstertarget _currentorder_requiredmineral _currentorder_weaponrow _currentorder_cost _currentorder_waittime) (break `/Game/InventorySystem/ItemData/Order/S_OrderData` (`self.CurrentOrder`)))
  (bind _output_get (set `self.WaitTimeMax` _currentorder_waittime))
  (bind _output_get_2 (set `self.WaitTimeCurrent	` _output_get))
  (bind _output_get_3 (set `self.IsCountingWaitTime` true))
  (`/Engine/EditorBlueprintResources/StandardMacros.IsValid` _orderdetailwidget
    (:`Is Valid`
      (`/Game/SmithShop/UI/WB_OrderDetail.SetOrderWaitTime` _orderdetailwidget _output_get_2 _output_get_3)
      (`Widget.SetIsEnabled` (`/Game/SmithShop/UI/WB_SlotandInventoryDisplay.CraftBtn` (`self.SlotAndInventory`)) true)
      (`Widget.SetIsEnabled` (`/Game/SmithShop/UI/WB_SlotandInventoryDisplay.swordBtn` (`self.SlotAndInventory`)) true)
      (`Widget.SetIsEnabled` (`/Game/SmithShop/UI/WB_SlotandInventoryDisplay.bowBtn` (`self.SlotAndInventory`)) true)
      (`Widget.SetIsEnabled` (`/Game/SmithShop/UI/WB_SlotandInventoryDisplay.staffBtn` (`self.SlotAndInventory`)) true))))

(event `self.ReceiveTick`
  (params (DeltaSeconds :type "Float (single-precision)"))
  (bind _returnvalue (`KismetMathLibrary.FClamp` (- (`/Game/SmithShop/UI/WB_TimerShop.RemainingTime` (`self.ShopTimerWidgetInstance`)) 20.0) 0.0 9999.0))
  (if (`self.IsCountingWaitTime`)
    (bind _output_get (set `self.WaitTimeCurrent	` (- (`self.WaitTimeCurrent	`) DeltaSeconds)))
    (if (<= _output_get 0.0)
      (set `self.IsCountingWaitTime` false)
      (bind _output_get_2 (set `self.ShopTime` _returnvalue))
      (if (== _returnvalue 0.0)
        (`self.EndShopSessioNew`)
        (else
          (`KismetSystemLibrary.K2_ClearAndInvalidateTimerHandle` (`self.ShopTimerHandle	`))
          (`/Game/SmithShop/UI/WB_TimerShop.RefreshRemainingTime` (`self.ShopTimerWidgetInstance`) _output_get_2)
          (bind _returnvalue_2 (`KismetSystemLibrary.K2_SetTimerDelegate` (delegate `EndShopSessioNew`) _output_get_2))
          (set `self.ShopTimerHandle	` _returnvalue_2))))))

(fn `FocusTarget`
  (returns (Message :type Text))
  (return (`|FormatText` "{Container}" (`self.ContainerName`))))

(fn `GetContainerData`
  (returns (ContainerData :type "/Game/SaveSystem/Structs/S_ContainerData Structure"))
  (bind _asbp_third_person_game_mode (cast `/Game/ThirdPerson/Blueprints/BP_ThirdPersonGameMode` (`GameplayStatics.GetGameMode`)))
  (bind _containerdata (`/Game/SaveSystem/BP_SaveData_Level.ContainerData` (`/Game/ThirdPerson/Blueprints/BP_ThirdPersonGameMode.SaveDataLevel` _asbp_third_person_game_mode)))
  (bind (_containers _containerinventories) (break `/Game/SaveSystem/Structs/S_ContainerData` _containerdata))
  (`KismetArrayLibrary.Array_Add` _containers (`|ConvertAsset` (`self.BPC_Inventory`)))
  (`KismetArrayLibrary.Array_Add` _containerinventories (make `/Game/SaveSystem/Structs/S_ContainerInventory` (`/Game/InventorySystem/BPC_Inventory.ItemSlots` (`self.BPC_Inventory`))))
  (return _containerdata))

(fn `GetRandomOrder`
  (params (S_OrderData :type "/Game/InventorySystem/ItemData/Order/S_OrderData Structure (by ref)"))
  (returns (NewParam :type "/Game/InventorySystem/ItemData/Order/S_OrderData Structure"))
  (bind _outrownames (`DataTableFunctionLibrary.GetDataTableRowNames` "/Game/InventorySystem/ItemData/Order/DT_OrderData.DT_OrderData"))
  (bind _returnvalue (`|GetDataTableRow` "/Game/InventorySystem/ItemData/Order/DT_OrderData.DT_OrderData" (`|GetArrayItem` _outrownames (`KismetMathLibrary.RandomIntegerInRange` 0 (- (`KismetArrayLibrary.Array_Length` _outrownames) 1))))
    (:`then`
      (`Widget.SetIsEnabled` (`/Game/SmithShop/UI/WB_OrderDetail.AcceptButton` (`self.OrderDetailWidget`)) true)
      (`Widget.SetIsEnabled` (`/Game/SmithShop/UI/WB_OrderDetail.DeclineButton` (`self.OrderDetailWidget`)) true)
      (bind (_adventureimage _weapontype _monstertarget _requiredmineral _weaponrow _cost _waittime _monsterimage _mineralpic) (break `/Game/InventorySystem/ItemData/Order/S_OrderData` _returnvalue))
      (return (make `/Game/InventorySystem/ItemData/Order/S_OrderData` _adventureimage _weapontype _monstertarget _requiredmineral _weaponrow _cost _waittime _monsterimage _mineralpic)))))

(fn `LoadContainerData`
  (params (ContainerData :type "/Game/SaveSystem/Structs/S_ContainerData Structure"))
  (bind (_containers _containerinventories) (break `/Game/SaveSystem/Structs/S_ContainerData` ContainerData))
  (bind _output_get (set `/Game/InventorySystem/BPC_Inventory.ItemSlots` (`.ContainerInventory_3_89E0B9F148EB77087CEDECADFF9980C7` (break `/Game/SaveSystem/Structs/S_ContainerInventory` (`|GetArrayItem` _containerinventories (`KismetArrayLibrary.Array_Find` _containers (`|ConvertAsset` (`self.BPC_Inventory`)))))) (`self.BPC_Inventory`)))
  (`KismetArrayLibrary.Array_Resize` _output_get (`self.ContainerSize`)))

(fn `SpawnNewOrderWidget `
  (returns (OrderDetailRef :type "/Game/SmithShop/UI/WB_OrderDetail Object Reference"))
  (bind _returnvalue (`|CreateWidget` "/Game/SmithShop/UI/WB_OrderDetail.WB_OrderDetail_C" (`GameplayStatics.GetPlayerController` 0) null))
  (bind _output_get (set `self.OrderDetailWidget` _returnvalue))
  (`UserWidget.AddToViewport` _output_get 1)
  (set `PlayerController.bShowMouseCursor` true (`GameplayStatics.GetPlayerController` 0))
  (add `/Game/SmithShop/UI/WB_OrderDetail.OnOrderAccepted` _output_get (`|CreateDelegate` :!event `HandleOrderAccepted`))
  (add `/Game/SmithShop/UI/WB_OrderDetail.OnOrderDeclined` _output_get (`|CreateDelegate` :!event `HandleOrderDeclined`))
  (bind _newparam (`self.GetRandomOrder` (`self.CurrentOrder`)))
  (bind _output_get_2 (set `self.CurrentOrder` _newparam))
  (`/Game/SmithShop/UI/WB_OrderDetail.UpdateUI` _output_get _output_get_2)
  (return _output_get))

(fn `UserConstructionScript`)