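; Smith shop trigger actor that lets the player open a timed shop session by pressing E inside its box.
; Box overlaps with BP_MainCharacter set the range flag that gates the key.
; Opening disables character input, shows timer and shop widgets, and fills the order detail with a random DT_OrderData row.
; A fixed-delay timer, separate from the ShopTime value shown, removes both widgets and restores input.
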(event `self.ReceiveBeginPlay`
  (`self.EnableInput` (`GameplayStatics.GetPlayerController` 0)))

(event `self.Box.OnComponentBeginOverlap`
  (params (OverlappedComponent :type "PrimitiveComponent Object Reference") (OtherActor :type "Actor Object Reference") (OtherComp :type "PrimitiveComponent Object Reference") (OtherBodyIndex :type Integer) (bFromSweep :type Boolean) (SweepResult :type "HitResult Structure (by ref)"))
  (cast `/Game/ThirdPerson/Blueprints/BP_MainCharacter` OtherActor)
  (set `self.IsPlayerInRange	` true))

(event `self.Box.OnComponentEndOverlap`
  (params (OverlappedComponent :type "PrimitiveComponent Object Reference") (OtherActor :type "Actor Object Reference") (OtherComp :type "PrimitiveComponent Object Reference") (OtherBodyIndex :type Integer))
  (cast `/Game/ThirdPerson/Blueprints/BP_MainCharacter` OtherActor)
  (set `self.IsPlayerInRange	` false))

(event `Key|E`
  (params (Key :type "Key Structure"))
  (:`Pressed`
    (if (`self.IsPlayerInRange	`)
      (if (not (`self.IsShopOpen`))
        (set `self.IsShopOpen` true)
        (bind _returnvalue (`KismetSystemLibrary.K2_SetTimerDelegate` (delegate `EndShopSession`) 5.0))
        (set `self.ShopTimerHandle	` _returnvalue)
        (bind _returnvalue_2 (`|CreateWidget` "/Game/SmithShop/UI/WB_TimerShop.WB_TimerShop_C" (`GameplayStatics.GetPlayerController` 0)))
        (bind _output_get (set `self.ShopTimerWidgetInstance` _returnvalue_2))
        (`UserWidget.AddToViewport` _output_get 0)
        (`self.DisableInput` (`GameplayStatics.GetPlayerCharacter` 0) (`GameplayStatics.GetPlayerController` 0))
        (set `/Game/SmithShop/UI/WB_TimerShop.RemainingTime` (`self.ShopTime`) (`self.ShopTimerWidgetInstance`))
        (bind _returnvalue_3 (`|CreateWidget` "/Game/SmithShop/UI/WB_FullShop.WB_FullShop_C" (`GameplayStatics.GetPlayerController` 0)))
        (bind _output_get_2 (set `self.FullShopWidget` _returnvalue_3))
        (`UserWidget.AddToViewport` _output_get_2 0)
        (bind _orderdata (`self.GetRandomOrder` (struct)))
        (`/Game/SmithShop/UI/WB_OrderDetail.UpdateUI` (`/Game/SmithShop/UI/WB_FullShop.WB_OrderDetail` _returnvalue_3) _orderdata)))))

(event `EndShopSession`
  (`Widget.RemoveFromParent` (`self.ShopTimerWidgetInstance`))
  (`Widget.RemoveFromParent` (`self.FullShopWidget`))
  (set `self.IsShopOpen` false)
  (`self.EnableInput` (`GameplayStatics.GetPlayerCharacter` 0) (`GameplayStatics.GetPlayerController` 0)))

(fn `GetRandomOrder`
  (params (S_OrderData :type "/Game/InventorySystem/ItemData/Order/S_OrderData Structure (by ref)"))
  (returns (OrderData :type "/Game/InventorySystem/ItemData/Order/S_OrderData Structure"))
  (bind _outrownames (`DataTableFunctionLibrary.GetDataTableRowNames` "/Game/InventorySystem/ItemData/Order/DT_OrderData.DT_OrderData"))
  (bind _returnvalue (`|GetDataTableRow` "/Game/InventorySystem/ItemData/Order/DT_OrderData.DT_OrderData" (`|GetArrayItem` _outrownames (`KismetMathLibrary.RandomIntegerInRange` 0 (- (`KismetArrayLibrary.Array_Length` _outrownames) 1))))
    (:`then`
      (bind (_adventureimage _weapontype _monstertarget _requiredmineral _weaponrow _cost _waittime) (break `/Game/InventorySystem/ItemData/Order/S_OrderData` _returnvalue))
      (return (make `/Game/InventorySystem/ItemData/Order/S_OrderData` _adventureimage _weapontype _monstertarget _requiredmineral _weaponrow _cost _waittime)))))

(fn `UserConstructionScript`)