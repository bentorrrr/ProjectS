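; BP_InventoryComponent holds the player's ten-slot item inventory and creates the WB_Inventory widget that displays it.
; The I key toggles the widget, while Q sphere-traces near the player character's feet for a BP_Item to pick up.
; Pickup scans slots in order, taking the first compatible stack (capped at 64) or empty slot, whichever comes first, then reloads the widget and destroys the item.
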(event `self.ReceiveBeginPlay`
  (bind _returnvalue (`|CreateWidget` "/Game/Inventory/Widgets/WB_Inventory.WB_Inventory_C"))
  (set `self.InventoryWidger` _returnvalue)
  (`KismetArrayLibrary.Array_Resize` (`self.Items`) 10)
  (`/Game/Inventory/Widgets/WB_Inventory.LoadInventory` (`self.InventoryWidger`) self))

(event `Key|I`
  (params (Key :type "Key Structure"))
  (bind _inventorywidger (`self.InventoryWidger`))
  (:`Pressed`
    (if (`Widget.IsVisible` (`self.InventoryWidger`))
      (`Widget.RemoveFromParent` _inventorywidger)
      (else
        (`UserWidget.AddToViewport` _inventorywidger 0)))))

(event `Key|Q`
  (params (Key :type "Key Structure"))
  (bind _returnvalue (- (`Actor.K2_GetActorLocation` (`GameplayStatics.GetPlayerCharacter` 0)) (0.0 0.0 65.0)))
  (:`Pressed`
    (bind _outhit (`KismetSystemLibrary.SphereTraceSingle` _returnvalue _returnvalue 120.0 "TraceTypeQuery1"))
    (bind _asbp_item (cast `/Game/Inventory/Blueprints/BP_Item` (`.HitActor` (`GameplayStatics.BreakHitResult` _outhit))))
    (for (_array_element _array_index) (`self.Items`)
      (`/Engine/EditorBlueprintResources/StandardMacros.IsValid` _asbp_item
        (:`Is Valid`
          (bind (_name _stackable _quantity) (break `/Game/Inventory/Blueprints/S_ItemStructure` _array_element))
          (bind (_name_2 _stackable_2 _quantity_2) (break `/Game/Inventory/Blueprints/S_ItemStructure` (`/Game/Inventory/Blueprints/BP_Item.Item` _asbp_item)))
          (bind _returnvalue_2 (+ _quantity _quantity_2))
          (if (and (`KismetTextLibrary.EqualEqual_TextText` _name _name_2) _stackable_2 (<= _returnvalue_2 64))
            (bind (_item_name _item_stackable _item_quantity _item_thumnail _item_mesh) (break `/Game/Inventory/Blueprints/S_ItemStructure` (`/Game/Inventory/Blueprints/BP_Item.Item` _asbp_item)))
            (`KismetArrayLibrary.Array_Set` (`self.Items`) _array_index (make `/Game/Inventory/Blueprints/S_ItemStructure` _item_name _item_stackable _returnvalue_2 _item_thumnail _item_mesh))
            (`/Game/Inventory/Widgets/WB_Inventory.LoadInventory` (`self.InventoryWidger`) self :!label _label)
            (`Actor.K2_DestroyActor` _asbp_item)
            (elif (== _quantity 0)
              (`KismetArrayLibrary.Array_Set` (`self.Items`) _array_index (`/Game/Inventory/Blueprints/BP_Item.Item` _asbp_item))
              (goto _label))))))))