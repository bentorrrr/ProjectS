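; Game instance that owns the save game and tracks the date, time of day, shop upgrade state and currency.
; On Init it loads the SaveData slot, or creates one starting on day 1 morning.
; Advancing time steps through five slots, rolling Night into the next day, with fade/UI widgets, saves including quests and inventory, and a level load.
; This sequence exists twice: a Delay-based event and a timer-by-name function.
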(event `self.ReceiveInit`
  (`/Game/SaveSystem/BPI_SaveSystem.LoadGameData`))

(event `/Game/SaveSystem/BPI_SaveSystem.LoadGameData`
  (bind _returnvalue (`GameplayStatics.DoesSaveGameExist` "SaveData"))
  (if _returnvalue
    (`self.LoadSaveData`)
    (else
      (bind _returnvalue_2 (`GameplayStatics.CreateSaveGameObject` "/Game/SaveSystem/MySaveData.MySaveData_C"))
      (set `self.SaveData` _returnvalue_2)
      (set `self.CurrentTimeSlot` "NewEnumerator0")
      (set `self.CurrentDate` 1))))

(event `/Game/SaveSystem/BPI_SaveSystem.SaveGameData`
  ;[1 1 1] Save Game Data
  (`GameplayStatics.SaveGameToSlot` (`self.SaveData`) "SaveData"))

(event `/Game/SaveSystem/BPI_SaveSystem.SavePlayerData`
  (params (InventoryData :type "Array of /Game/InventorySystem/ItemData/item/S_ItemSlot Structure (by ref)"))
  ;[1 1 1] Save Player Data
  (set `/Game/SaveSystem/MySaveData.InventoryData` InventoryData (`self.SaveData`))
  (`/Game/SaveSystem/BPI_SaveSystem.SaveGameData`))

(event `AdvancingTimeSlot`
  (bind _playercharacter (`/Game/QuestSystem/Interaction/BPFL_CommonFunction.GetMainPlayerCharacter`))
  (bind _playercharacter_2 (`/Game/QuestSystem/Interaction/BPFL_CommonFunction.GetMainPlayerCharacter`))
  (bind _savedata (`self.SaveData`))
  (bind _savedata_2 (`self.SaveData`))
  ;[1 1 1] Advance Timeslot
  (switch `/Game/Utils/E_TimeSlot` (`self.CurrentTimeSlot`)
    (:`NewEnumerator0`
      (set `self.CurrentTimeSlot` "NewEnumerator1")
      (bind _currenttimeslot (`self.GetCurrentTimeSlot` :!label _label))
      (bind _returnvalue (`|CreateWidget` "/Game/Menu/WB_Fade.WB_Fade_C"))
      (`UserWidget.AddToViewport` _returnvalue 0)
      (`/Game/Menu/WB_Fade.PlayFadeIn` _returnvalue)
      (`KismetSystemLibrary.Delay` 2.0)
      (bind _returnvalue_2 (`|CreateWidget` "/Game/Utils/WB_TimeSlotUI.WB_TimeSlotUI_C"))
      (`UserWidget.AddToViewport` _returnvalue_2 0)
      (`/Game/Utils/WB_TimeSlotUI.TimeSlotUI` _returnvalue_2 _currenttimeslot)
      (`KismetSystemLibrary.Delay` 2.0)
      (`/Game/SaveSystem/MySaveData.SaveTimeSlots` (`self.SaveData`) (`self.CurrentDate`) (`self.CurrentTimeSlot`))
      (for _array_element (`/Game/QuestSystem/AC_QuestLog.CurrentQuests` (`/Game/ThirdPerson/Blueprints/BP_MainCharacter.AC_QuestLog` _playercharacter_2))
        (`/Game/SaveSystem/MySaveData.SaveQuestDetails` (`self.SaveData`) _array_element))
      (`self.SavePlayerData` (`/Game/InventorySystem/BPC_Inventory.GetInventoryData` (`/Game/ThirdPerson/Blueprints/BP_MainCharacter.BPC_Inventory` _playercharacter_2)))
      (`/Game/SaveSystem/MySaveData.SaveQuestLog` (`self.SaveData`) (`/Game/ThirdPerson/Blueprints/BP_MainCharacter.AC_QuestLog` (`/Game/QuestSystem/Interaction/BPFL_CommonFunction.GetMainPlayerCharacter`)))
      (`/Game/SaveSystem/BP_SaveLibrary.SaveSFX`)
      (`/Game/SaveSystem/BP_SaveLibrary.SavePlayerData`)
      (`/Game/SaveSystem/MySaveData.SaveShopComponents` _savedata_2 (`self.LevelUpgrade`) (`self.UpgradeCost`))
      (`/Game/SaveSystem/MySaveData.SavePlayerCurrency` _savedata_2 (`self.PlayerCurrency`))
      (`GameplayStatics.SaveGameToSlot` (`self.SaveData`) "SaveData")
      (bind _returnvalue_3 (`|CreateWidget` "/Game/Menu/WB_Fade.WB_Fade_C"))
      (`UserWidget.AddToViewport` _returnvalue_3 0)
      (`/Game/Menu/WB_Fade.PlayFadeIn` _returnvalue_3)
      (`KismetSystemLibrary.Delay` 2.0)
      (`GameplayStatics.OpenLevelBySoftObjectPtr` "/Game/ThirdPerson/Maps/Town.Town"))
    (:`NewEnumerator1`
      (set `self.CurrentTimeSlot` "NewEnumerator2")
      (goto _label))
    (:`NewEnumerator2`
      (set `self.CurrentTimeSlot` "NewEnumerator3")
      (goto _label))
    (:`NewEnumerator3`
      (set `self.CurrentTimeSlot` "NewEnumerator4")
      (goto _label))
    (:`NewEnumerator4`
      (`self.AdvanceDate`)
      (bind _returnvalue_4 (`|CreateWidget` "/Game/Menu/WB_Fade.WB_Fade_C"))
      (`UserWidget.AddToViewport` _returnvalue_4 0)
      (`/Game/Menu/WB_Fade.PlayFadeIn` _returnvalue_4)
      (`KismetSystemLibrary.Delay` 2.0)
      (bind _returnvalue_5 (`|CreateWidget` "/Game/Utils/WB_DateChange.WB_DateChange_C"))
      (`UserWidget.AddToViewport` _returnvalue_5 0)
      (`/Game/Utils/WB_DateChange.ChangeDateUI` _returnvalue_5 (`self.CurrentDate`))
      (`KismetSystemLibrary.Delay` 2.0)
      (bind _returnvalue_6 (`|CreateWidget` "/Game/Menu/WB_Fade.WB_Fade_C"))
      (`UserWidget.AddToViewport` _returnvalue_6 0)
      (`/Game/Menu/WB_Fade.PlayFadeIn` _returnvalue_6)
      (`KismetSystemLibrary.Delay` 2.0)
      (bind _output_get (set `self.CurrentTimeSlot` "NewEnumerator0"))
      (bind _returnvalue_7 (`|CreateWidget` "/Game/Utils/WB_TimeSlotUI.WB_TimeSlotUI_C"))
      (`UserWidget.AddToViewport` _returnvalue_7 0)
      (`/Game/Utils/WB_TimeSlotUI.TimeSlotUI` _returnvalue_7 _output_get)
      (`KismetSystemLibrary.Delay` 2.0)
      (bind _returnvalue_8 (`|CreateWidget` "/Game/Menu/WB_Fade.WB_Fade_C"))
      (`UserWidget.AddToViewport` _returnvalue_8 0)
      (`/Game/Menu/WB_Fade.PlayFadeIn` _returnvalue_8)
      (`/Game/SaveSystem/MySaveData.SaveTimeSlots` (`self.SaveData`) (`self.CurrentDate`) (`self.CurrentTimeSlot`))
      (for _array_element_2 (`/Game/QuestSystem/AC_QuestLog.CurrentQuests` (`/Game/ThirdPerson/Blueprints/BP_MainCharacter.AC_QuestLog` _playercharacter))
        (`/Game/SaveSystem/MySaveData.SaveQuestDetails` (`self.SaveData`) _array_element_2))
      (`self.SavePlayerData` (`/Game/InventorySystem/BPC_Inventory.GetInventoryData` (`/Game/ThirdPerson/Blueprints/BP_MainCharacter.BPC_Inventory` _playercharacter)))
      (`/Game/SaveSystem/MySaveData.SaveQuestLog` (`self.SaveData`) (`/Game/ThirdPerson/Blueprints/BP_MainCharacter.AC_QuestLog` (`/Game/QuestSystem/Interaction/BPFL_CommonFunction.GetMainPlayerCharacter`)))
      (`/Game/SaveSystem/BP_SaveLibrary.SaveSFX`)
      (`/Game/SaveSystem/BP_SaveLibrary.SavePlayerData`)
      (`/Game/SaveSystem/MySaveData.SaveShopComponents` _savedata (`self.LevelUpgrade`) (`self.UpgradeCost`))
      (`/Game/SaveSystem/MySaveData.SavePlayerCurrency` _savedata (`self.PlayerCurrency`))
      (`GameplayStatics.SaveGameToSlot` (`self.SaveData`) "SaveData")
      (`KismetSystemLibrary.Delay` 2.0)
      (`GameplayStatics.OpenLevelBySoftObjectPtr` "/Game/ThirdPerson/Maps/Town.Town"))))

(fn `AdvanceDate`
  (returns (CurrentDate :type Integer))
  (bind _output_get (set `self.CurrentDate` (+ (`self.CurrentDate`) 1)))
  (return _output_get))

(fn `AdvanceTimeSlot`
  (returns (CurrentTimeSlot :type "/Game/Utils/E_TimeSlot Enum"))
  (bind _playercharacter (`/Game/QuestSystem/Interaction/BPFL_CommonFunction.GetMainPlayerCharacter`))
  (bind _playercharacter_2 (`/Game/QuestSystem/Interaction/BPFL_CommonFunction.GetMainPlayerCharacter`))
  (bind _savedata (`self.SaveData`))
  (bind _savedata_2 (`self.SaveData`))
  (switch `/Game/Utils/E_TimeSlot` (`self.CurrentTimeSlot`)
    (:`NewEnumerator0`
      (set `self.CurrentTimeSlot` "NewEnumerator1"))
    (:`NewEnumerator1`
      (set `self.CurrentTimeSlot` "NewEnumerator2"))
    (:`NewEnumerator2`
      (set `self.CurrentTimeSlot` "NewEnumerator3"))
    (:`NewEnumerator3`
      (set `self.CurrentTimeSlot` "NewEnumerator4"))
    (:`NewEnumerator4`
      (`self.AdvanceDate`)
      (bind _returnvalue (`|CreateWidget` "/Game/Menu/WB_Fade.WB_Fade_C"))
      (`UserWidget.AddToViewport` _returnvalue 0)
      (`/Game/Menu/WB_Fade.PlayFadeIn` _returnvalue)
      (`KismetSystemLibrary.K2_SetTimer` null "OpenDateChangeUI" 2.0)
      (`KismetSystemLibrary.K2_SetTimer` null "FadeIn" 4.0)
      (`KismetSystemLibrary.K2_SetTimer` null "OpenTimeSlotUI" 6.0)
      (set `self.CurrentTimeSlot` "NewEnumerator0")
      (bind _currenttimeslot (`self.GetCurrentTimeSlot`))
      (bind _returnvalue_2 (`|CreateWidget` "/Game/Menu/WB_Fade.WB_Fade_C"))
      (`UserWidget.AddToViewport` _returnvalue_2 0)
      (`/Game/Menu/WB_Fade.PlayFadeIn` _returnvalue_2)
      (`/Game/SaveSystem/MySaveData.SaveTimeSlots` (`self.SaveData`) (`self.CurrentDate`) _currenttimeslot)
      (for _array_element (`/Game/QuestSystem/AC_QuestLog.CurrentQuests` (`/Game/ThirdPerson/Blueprints/BP_MainCharacter.AC_QuestLog` _playercharacter))
        (`/Game/SaveSystem/MySaveData.SaveQuestDetails` (`self.SaveData`) _array_element))
      (`self.SavePlayerData` (`/Game/InventorySystem/BPC_Inventory.GetInventoryData` (`/Game/ThirdPerson/Blueprints/BP_MainCharacter.BPC_Inventory` _playercharacter)))
      (`/Game/SaveSystem/MySaveData.SaveQuestLog` (`self.SaveData`) (`/Game/ThirdPerson/Blueprints/BP_MainCharacter.AC_QuestLog` (`/Game/QuestSystem/Interaction/BPFL_CommonFunction.GetMainPlayerCharacter`)))
      (`/Game/SaveSystem/BP_SaveLibrary.SaveSFX`)
      (`/Game/SaveSystem/BP_SaveLibrary.SavePlayerData`)
      (`/Game/SaveSystem/BP_SaveLibrary.SaveLevelData`)
      (`/Game/SaveSystem/MySaveData.SaveShopComponents` _savedata (`self.LevelUpgrade`) (`self.UpgradeCost`))
      (`/Game/SaveSystem/MySaveData.SavePlayerCurrency` _savedata (`self.PlayerCurrency`))
      (`GameplayStatics.SaveGameToSlot` (`self.SaveData`) "SaveData")
      (`KismetSystemLibrary.K2_SetTimer` null "FadeIn" 8.0)
      (`KismetSystemLibrary.K2_SetTimer` null "LoadLevel" 10.0)
      (return _currenttimeslot)))
  (bind _currenttimeslot_2 (`self.GetCurrentTimeSlot`))
  (bind _returnvalue_3 (`|CreateWidget` "/Game/Menu/WB_Fade.WB_Fade_C"))
  (`UserWidget.AddToViewport` _returnvalue_3 0)
  (`/Game/Menu/WB_Fade.PlayFadeIn` _returnvalue_3)
  (`KismetSystemLibrary.K2_SetTimer` null "OpenTimeSlotUI" 2.0)
  (`KismetSystemLibrary.K2_SetTimer` null "FadeIn" 4.0)
  (`/Game/SaveSystem/MySaveData.SaveTimeSlots` (`self.SaveData`) (`self.CurrentDate`) _currenttimeslot_2)
  (for _array_element_2 (`/Game/QuestSystem/AC_QuestLog.CurrentQuests` (`/Game/ThirdPerson/Blueprints/BP_MainCharacter.AC_QuestLog` _playercharacter_2))
    (`/Game/SaveSystem/MySaveData.SaveQuestDetails` (`self.SaveData`) _array_element_2))
  (`self.SavePlayerData` (`/Game/InventorySystem/BPC_Inventory.GetInventoryData` (`/Game/ThirdPerson/Blueprints/BP_MainCharacter.BPC_Inventory` _playercharacter_2)))
  (`/Game/SaveSystem/MySaveData.SaveQuestLog` (`self.SaveData`) (`/Game/ThirdPerson/Blueprints/BP_MainCharacter.AC_QuestLog` (`/Game/QuestSystem/Interaction/BPFL_CommonFunction.GetMainPlayerCharacter`)))
  (`/Game/SaveSystem/BP_SaveLibrary.SaveSFX`)
  (`/Game/SaveSystem/BP_SaveLibrary.SavePlayerData`)
  (`/Game/SaveSystem/BP_SaveLibrary.SaveLevelData`)
  (`/Game/SaveSystem/MySaveData.SaveShopComponents` _savedata_2 (`self.LevelUpgrade`) (`self.UpgradeCost`))
  (`/Game/SaveSystem/MySaveData.SavePlayerCurrency` _savedata_2 (`self.PlayerCurrency`))
  (`GameplayStatics.SaveGameToSlot` (`self.SaveData`) "SaveData")
  (`/Game/Menu/WB_Fade.PlayFadeIn` _returnvalue_3)
  (`KismetSystemLibrary.K2_SetTimer` null "LoadLevel" 6.0)
  (return _currenttimeslot_2))

(fn `GetCurrentDate`
  (returns (CurrentDate :type Integer))
  (return (`self.CurrentDate`)))

(fn `GetCurrentTimeSlot`
  (returns (CurrentTimeSlot :type "/Game/Utils/E_TimeSlot Enum"))
  (return (`self.CurrentTimeSlot`)))

(fn `GetSaveData`
  (returns (SaveData :type "/Game/SaveSystem/Structs/S_SaveData Structure"))
  (return (make `/Game/SaveSystem/Structs/S_SaveData` (`self.SaveData`) null)))

(fn `LoadSaveData`
  (bind _returnvalue (`GameplayStatics.LoadGameFromSlot` "SaveData"))
  (bind _asmy_save_data (cast `/Game/SaveSystem/MySaveData` _returnvalue))
  (bind _output_get (set `self.SaveData` _asmy_save_data))
  (`/Game/SaveSystem/MySaveData.LoadTimeSlots` _output_get self)
  (`/Game/SaveSystem/MySaveData.LoadShopComponents` _output_get self)
  (`/Game/SaveSystem/MySaveData.LoadPlayerCurrency` _output_get self))